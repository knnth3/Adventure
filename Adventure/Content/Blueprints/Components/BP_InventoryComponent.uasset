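; Inventory component that shows equipped items as actors held in the owner's hands; added, removed and overburdened events are empty stubs.
; On BeginPlay it caches the owner's first skeletal mesh with a configured tag.
; Equipping looks up the object enum in a held-objects DataTable, spawns its class and snaps it to a hand socket, swapping hands if LeftHanded.
; Unequipping destroys the held actor, always treating right as main hand.
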(event `self.ReceiveBeginPlay`
  (`self.PreLoadSettings`))

(event `self.OnObjectEquiped`
  (params (objectEnum :type Byte) (bInMainHand :type Boolean))
  ;[1 1 1] Equip
  (`/Engine/EditorBlueprintResources/StandardMacros.IsValid` (`self.ParentSkeletalMesh`)
    (:`Is Valid`
      (bind _returnvalue (`|GetDataTableRow` "/Game/Blueprints/HeldObjects/Table_HeldObjects.Table_HeldObjects" (`KismetStringLibrary.Conv_StringToName` (`KismetStringLibrary.Conv_ByteToString` objectEnum)))
        (:`then`
          (`self.SpawnHeldObject` (`.Class_12_5F86F4DB447313C3C1880D80046C1B9B` (break `/Game/Blueprints/HeldObjects/Struct_HeldObject` _returnvalue)) bInMainHand))))))

(event `self.OnObjectUnequiped`
  (params (bInMainHand :type Boolean))
  (bind _rhandobject (`self.RHandObject`))
  (bind _lhandobject (`self.LHandObject`))
  ;[1 1 1] Unequip
  (if bInMainHand
    (`/Engine/EditorBlueprintResources/StandardMacros.IsValid` _rhandobject
      (:`Is Valid`
        (`Actor.K2_DestroyActor` _rhandobject)
        (set `self.RHandObject` null)))
    (else
      (`/Engine/EditorBlueprintResources/StandardMacros.IsValid` _lhandobject
        (:`Is Valid`
          (`Actor.K2_DestroyActor` _lhandobject)
          (set `self.LHandObject` null))))))

(event `self.OnObjectAdded`
  (params (objectEnum :type Byte)))

(event `self.OnObjectRemoved`
  (params (objectEnum :type Byte)))

(event `self.OnBecomeOverburdened`
  (params (newState :type Boolean)))

(fn `PreLoadSettings`
  (bind _returnvalue (`Actor.GetComponentsByTag` (`self.GetOwner`) "/Script/Engine.SkeletalMeshComponent" (`self.SkeletalMeshTag`)))
  (if (!= (`KismetArrayLibrary.Array_Length` _returnvalue) 0)
    (set `self.ParentSkeletalMesh` (`|GetArrayItem` _returnvalue))
    (else
      (`KismetSystemLibrary.PrintString` "Could not find a suitable skeletal mesh to spawn equiped items"))))

(fn `SpawnHeldObject`
  (params (Class :type "/Game/Blueprints/HeldObjects/BP_HeldObject Class Reference") (bInMainHand :type Boolean))
  (locals (DefaultTransform :type "Transform Structure" :default "0.000000,0.000000,0.000000|0.000000,0.000000,0.000000|1.000000,1.000000,1.000000") (NewActor :type "/Game/Blueprints/HeldObjects/BP_HeldObject Object Reference"))
  (bind _blefthanded (`self.bLeftHanded`))
  (bind _newactor (`local.NewActor`))
  (bind _newactor_2 (`local.NewActor`))
  (if (!= Class null)
    (bind _returnvalue (`|SpawnActorFromClass` Class (`local.DefaultTransform`) "AlwaysSpawn" "OverrideRootScale" null null))
    (set `local.NewActor` _returnvalue)
    (if bInMainHand
      (if _blefthanded
        (set `self.LHandObject` _newactor_2)
        (`SceneComponent.K2_AttachToComponent` (`Actor.RootComponent` (`self.LHandObject`)) (`self.ParentSkeletalMesh`) (`self.LHand_Socket`) "SnapToTarget" "SnapToTarget" "SnapToTarget" true :!label _label)
        (else
          (set `self.RHandObject` _newactor_2)
          (`SceneComponent.K2_AttachToComponent` (`Actor.RootComponent` (`self.RHandObject`)) (`self.ParentSkeletalMesh`) (`self.RHand_Socket`) "SnapToTarget" "SnapToTarget" "SnapToTarget" true :!label _label_2)))
      (elif _blefthanded
        (set `self.RHandObject` _newactor)
        (goto _label_2)
        (else
          (set `self.LHandObject` _newactor)
          (goto _label))))
    (else
      (`KismetSystemLibrary.PrintString` "Object doesnt have a visual class, thus cannot be held"))))