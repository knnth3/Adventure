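; BP_PS_Multiplayer is a multiplayer player state that updates the HUD status text to reflect turn state.
; On a state change, it sets the first player controller's HUD_Multiplayer to free-roam, standby or active-turn text.
; Standby names the active player from BP_GS_Multiplayer, with a generic fallback if that cast fails.
; The active branch also casts the pawn to BP_ConnectedPlayer but does nothing further with it.
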(event `self.OnStateChanged`
  ;[1 1 1] Handle State Change
  (bind _ashud_multiplayer (cast `/Game/Blueprints/UI/Multiplayer/HUD_Multiplayer` (`PlayerController.GetHUD` (`GameplayStatics.GetPlayerController` 0))))
  (switch `TURN_BASED_STATE` (`self.GetCurrentState`)
    (:`FREE_ROAM`
      (`/Game/Blueprints/UI/Multiplayer/HUD_Multiplayer.SetStatus` _ashud_multiplayer "Free-Roam"))
    (:`STANDBY`
      (bind _asbp_gs_multiplayer (cast `/Game/Blueprints/GameStates/BP_GS_Multiplayer` (`GameplayStatics.GetGameState`))
        (:`then`
          (`/Game/Blueprints/UI/Multiplayer/HUD_Multiplayer.SetStatus` _ashud_multiplayer (`KismetStringLibrary.Concat_StrStr` (`GS_Multiplayer.GetActivePlayerName` _asbp_gs_multiplayer) "'s Turn")))
        (:`CastFailed`
          (`/Game/Blueprints/UI/Multiplayer/HUD_Multiplayer.SetStatus` _ashud_multiplayer "Standby..."))))
    (:`ACTIVE`
      (`/Game/Blueprints/UI/Multiplayer/HUD_Multiplayer.SetStatus` _ashud_multiplayer "Your Turn")
      (cast `/Game/Blueprints/Actors/BP_ConnectedPlayer` (`GameplayStatics.GetPlayerPawn` 0)))))

(fn `UserConstructionScript`)