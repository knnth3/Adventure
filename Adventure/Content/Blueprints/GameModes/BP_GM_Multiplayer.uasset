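; Multiplayer game mode Blueprint that handles requests to load a saved map from a save slot.
; OnLoadMapRequest creates a LevelSaveGame object, loads the slot, sets the grid dimensions from the saved map size and queues each saved object for pre-initialization.
; It returns whether the load succeeded and prints the loaded object count or a failure message.
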(fn `OnLoadMapRequest`
  (params (SaveSlot :type String))
  (returns (ReturnValue :type Boolean))
  (bind _returnvalue (`GameplayStatics.CreateSaveGameObject` "/Game/Blueprints/SaveGameFiles/LevelSaveGame.LevelSaveGame_C"))
  (bind _success (`/Game/Blueprints/SaveGameFiles/LevelSaveGame.Load` _returnvalue SaveSlot))
  (if _success
    (`self.SetGridDimensions` (`/Game/Blueprints/SaveGameFiles/LevelSaveGame.MapSize` _returnvalue))
    (bind _objects (`/Game/Blueprints/SaveGameFiles/LevelSaveGame.Objects` _returnvalue))
    (for _array_element _objects
      (`self.AddObjectForPreInit` _array_element))
    (`KismetSystemLibrary.PrintString` (`KismetStringLibrary.Concat_StrStr` "Loaded  " (`KismetStringLibrary.Conv_IntToString` (`KismetArrayLibrary.Array_Length` _objects)) "objects"))
    (return true)
    (else
      (`KismetSystemLibrary.PrintString` "Failed to load Map")
      (return false))))

(fn `UserConstructionScript`)