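; BP_WalkableCell is a grid cell marker that visualizes walkable range through its material's color and opacity.
; On BeginPlay it checks box overlaps, turning black for a tagged Character or red for a PathBlock.
; Overlapping a BP_WalkableArea activates it, with peak opacity falling as cell cost rises relative to radius.
; Tick lerps opacity in, or out after StartFadeAnimation until the actor destroys itself; other overlaps during fade-out destroy it immediately.
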(event `self.ReceiveBeginPlay`
  (bind _staticmesh (`self.StaticMesh`))
  (bind _outcomponents (`KismetSystemLibrary.ComponentOverlapComponents` (`self.Box`) (`self.GetTransform`) (`|MakeArray` "ObjectTypeQuery2" :!type "EObjectTypeQuery Enum") null (`|MakeArray` self :!type "Actor Object Reference")))
  (for _array_element _outcomponents
    (if (`self.bCheckedForOverlap`)
      _
      (elif (`ActorComponent.ComponentHasTag` _array_element "Character")
        (`MeshComponent.SetVectorParameterValueOnMaterials` _staticmesh "Color" (0.0 0.0 0.0))
        (set `self.bCheckedForOverlap` true :!label _label)
        (elif (`ActorComponent.ComponentHasTag` _array_element "PathBlock")
          (`MeshComponent.SetVectorParameterValueOnMaterials` _staticmesh "Color" (1.0 0.0 0.0))
          (goto _label))))))

(event `self.ReceiveTick`
  (params (DeltaSeconds :type "Float (single-precision)"))
  (if (`self.bStartFadeAnim`)
    (bind _output_get (set `self.CurrentOpacity` (`KismetMathLibrary.Lerp` (`self.CurrentOpacity`) 0.0 (`self.DecayRate`))))
    (if (<= _output_get 0.01)
      (set `self.bStartFadeAnim` false)
      (set `self.bActivated` false)
      (`self.K2_DestroyActor`)
      (else
        (`MeshComponent.SetScalarParameterValueOnMaterials` (`self.StaticMesh`) "Opacity" _output_get)))
    (elif (`self.bActivated`)
      (bind _output_get_2 (set `self.CurrentOpacity` (`KismetMathLibrary.Lerp` (`self.CurrentOpacity`) (`self.MaxOpacity`) (`self.GrowthRate`))))
      (`MeshComponent.SetScalarParameterValueOnMaterials` (`self.StaticMesh`) "Opacity" _output_get_2))))

(event `self.Box.OnComponentBeginOverlap`
  (params (OverlappedComponent :type "PrimitiveComponent Object Reference") (OtherActor :type "Actor Object Reference") (OtherComp :type "PrimitiveComponent Object Reference") (OtherBodyIndex :type Integer) (bFromSweep :type Boolean) (SweepResult :type "HitResult Structure (by ref)"))
  (bind _asbp_walkable_area (cast `/Game/Blueprints/Grid/BP_WalkableArea` OtherActor)
    (:`then`
      (if (not (`self.bActivated`))
        (set `self.bActivated` true)
        (set `self.MaxOpacity` (+ 0.05 (* (- 1.0 (/ (* (`KismetMathLibrary.Conv_IntToDouble` (`/Game/Blueprints/Grid/BP_WalkableArea.GetCellCost` _asbp_walkable_area (`GridFunctions.WorldToGridLocation` (`self.K2_GetActorLocation` OtherActor)) (`GridFunctions.WorldToGridLocation` (`self.K2_GetActorLocation`)))) 0.1) (`KismetMathLibrary.Conv_IntToDouble` (`/Game/Blueprints/Grid/BP_WalkableArea.GetRadius` _asbp_walkable_area)))) 0.25)))))
    (:`CastFailed`
      (if (`self.bStartFadeAnim`)
        (`self.K2_DestroyActor`)))))

(fn `StartFadeAnimation`
  (set `self.bStartFadeAnim` true))

(fn `UserConstructionScript`)