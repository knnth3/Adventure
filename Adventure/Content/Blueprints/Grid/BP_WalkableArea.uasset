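; BP_WalkableArea displays the grid area within movement range of a center point as spawned BP_WalkableCell actors.
; GenerateArea spawns cells that are inside map bounds and within Radius, weighting diagonal steps 1.5 times straight ones.
; Tick expands an accelerating wave stage by stage, using radial damage as the signal that activates cells, with a brief delay between stages.
; DestroyArea starts each cell's fade and clears the list.
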(event `self.ReceiveTick`
  (params (DeltaSeconds :type "Float (single-precision)"))
  (`self.DelayTimer` DeltaSeconds 0.03
    (:`Finished`
      (if (`self.bAnimating`)
        (bind _output_get (set `self.ElapsedTime` (+ DeltaSeconds (`self.ElapsedTime`))))
        (bind (_remainder _returnvalue) (`KismetMathLibrary.FMod` (`self.GetDistanceTraveled` _output_get (`self.SpreadAcceleration`) 100.0) 152.399994))
        (if (> _returnvalue (`self.CurrentStage`))
          (bind _output_get_2 (set `self.CurrentStage` _returnvalue))
          (`self.ActivateCells` _output_get_2)
          (if (>= _output_get_2 (`self.Radius`))
            (set `self.CurrentStage` 0)
            (set `self.bAnimating` false)
            (set `self.ElapsedTime` 0.0)
            (else
              (set `self.bUseDelay` true))))))))

(fn `ActivateCells`
  (params (Radius :type Integer))
  (bind _returnvalue (`KismetMathLibrary.Conv_IntToDouble` Radius))
  (`GameplayStatics.ApplyRadialDamage` :`BaseDamage` _returnvalue :`Origin` (`self.CenterPoint`) :`DamageRadius` (* _returnvalue 153.0) :`DamageCauser` self :`InstigatedByController` null :`bDoFullDamage` true :`DamagePreventionChannel` "ECC_GameTraceChannel1"))

(fn `DestroyArea`
  (bind _cellactors (`self.CellActors`))
  (for _array_element _cellactors
    (`/Game/Blueprints/Grid/BP_WalkableCell.StartFadeAnimation` _array_element))
  (`KismetArrayLibrary.Array_Clear` _cellactors)
  (set `self.bActivated` false))

(fn `GenerateArea`
  (params (`Center Point` :type "GridCoordinate Structure") (Radius :type Integer) (TopLeftMap :type "GridCoordinate Structure") (BottomRightMap :type "GridCoordinate Structure"))
  (bind _returnvalue (* Radius 2))
  (for _index (range (+ _returnvalue 1))
    (for _index_2 (range (+ _returnvalue 1))
      (bind _returnvalue_2 (+ _index (- `Center Point_X` Radius)))
      (bind _returnvalue_3 (+ _index_2 (- `Center Point_Y` Radius)))
      (if (and (<= (* (`KismetMathLibrary.Conv_IntToDouble` (`self.GetCellCost` (make `GridCoordinate` `Center Point_X` `Center Point_Y`) (make `GridCoordinate` _returnvalue_2 _returnvalue_3))) 0.1) (`KismetMathLibrary.Conv_IntToDouble` Radius)) (`self.InBounds` TopLeftMap BottomRightMap (make `GridCoordinate` _returnvalue_2 _returnvalue_3)))
        (bind _returnvalue_4 (`|SpawnActorFromClass` "/Game/Blueprints/Grid/BP_WalkableCell.BP_WalkableCell_C" (`KismetMathLibrary.MakeTransform` (`GridFunctions.GridToWorldLocation` (make `GridCoordinate` _returnvalue_2 _returnvalue_3))) "AlwaysSpawn" "OverrideRootScale" null null))
        (`KismetArrayLibrary.Array_Add` (`self.CellActors`) _returnvalue_4))))
  (set `self.Radius` Radius)
  (set `self.bAnimating` true)
  (set `self.CurrentStage` 0)
  (set `self.ElapsedTime` 0.0)
  (set `self.CenterPoint` (`GridFunctions.GridToWorldLocation` (make `GridCoordinate` `Center Point_X` `Center Point_Y`)))
  (set `self.bActivated` true)
  (return))

(fn `GetCellCost`
  (params (Center :type "GridCoordinate Structure") (`Cell Location` :type "GridCoordinate Structure"))
  (returns (cost :type Integer))
  (bind _returnvalue (`KismetMathLibrary.Abs_Int` (- Center_Y `Cell Location_Y`)))
  (bind _returnvalue_2 (`KismetMathLibrary.Abs_Int` (- Center_X `Cell Location_X`)))
  (if (> _returnvalue_2 _returnvalue)
    (return (+ (* _returnvalue 15) (* (- _returnvalue_2 _returnvalue) 10)))
    (else
      (return (+ (* _returnvalue_2 15) (* (- _returnvalue _returnvalue_2) 10))))))

(fn `GetRadius`
  (returns (Radius :type Integer))
  (return (`self.Radius`)))

(fn `InBounds`
  (params (TopLeft :type "GridCoordinate Structure") (BottomRight :type "GridCoordinate Structure") (Coordinate :type "GridCoordinate Structure"))
  (returns (return :type Boolean))
  (return (and (`KismetMathLibrary.InRange_IntInt` Coordinate_X TopLeft_X BottomRight_X true false) (`KismetMathLibrary.InRange_IntInt` Coordinate_Y TopLeft_Y BottomRight_Y true false))))

(fn `IsActive`
  (returns (return :type Boolean))
  (return (`self.bActivated`)))

(fn `UserConstructionScript`)