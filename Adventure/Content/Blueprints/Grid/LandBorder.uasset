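; LandBorder is a grid actor that forms a scaled land border around a play grid of variable size.
; On BeginPlay, the TopLeft, BottomLeft and BottomRight pieces scale to the border dimensions plus one, in cell units.
; ConstructBorder offsets the Top, Right and TopRight pieces by the grid's world size, then stretches three Corner pieces from the grid and border dimensions, using a hard-coded cell factor on X and Y.
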(event `self.ReceiveBeginPlay`
  (bind _returnvalue (* (+ (`self.BorderDimensions`) 1.0) (`self.CellDimensions`)))
  (`SceneComponent.SetWorldScale3D` (`self.TopLeft`) _returnvalue)
  (`SceneComponent.SetWorldScale3D` (`self.BottomLeft`) _returnvalue)
  (`SceneComponent.SetWorldScale3D` (`self.BottomRight`) _returnvalue))

(fn `ConstructBorder`
  (params (GridDimensions :type "GridCoordinate Structure"))
  (bind (_x _y) (break `GridCoordinate` GridDimensions))
  (bind (_returnvalue_x _returnvalue_y) (`KismetMathLibrary.BreakVector` (`GridFunctions.GridToWorldLocation` GridDimensions)))
  (bind (_celldimensions_x _celldimensions_y _celldimensions_z) (`KismetMathLibrary.BreakVector` (`self.CellDimensions`)))
  (bind (_returnvalue_x_2 _returnvalue_y_2 _returnvalue_z) (`KismetMathLibrary.BreakVector` (+ (`self.BorderDimensions`) 1)))
  (bind _returnvalue (* _returnvalue_z _celldimensions_z))
  (bind _returnvalue_2 (* (`KismetMathLibrary.Conv_IntToDouble` (- (`KismetMathLibrary.FTrunc` _returnvalue_y_2) _y)) 1.524))
  (bind _returnvalue_3 (* (`KismetMathLibrary.Conv_IntToDouble` (- (`KismetMathLibrary.FTrunc` _returnvalue_x_2) _x)) 1.524))
  (`|ExecutionSequence`
    (:`then_0`
      (`SceneComponent.K2_AddWorldOffset` (`self.Top`) (`KismetMathLibrary.MakeVector` _returnvalue_x) false false)
      (`SceneComponent.K2_AddWorldOffset` (`self.Right`) (`KismetMathLibrary.MakeVector` 0.0 _returnvalue_y) false false)
      (`SceneComponent.K2_AddWorldOffset` (`self.TopRight`) (`KismetMathLibrary.MakeVector` _returnvalue_x _returnvalue_y) false false))
    (:`then_1`
      (`SceneComponent.SetWorldScale3D` (`self.CornerT`) (`KismetMathLibrary.MakeVector` _returnvalue_3 (* (`KismetMathLibrary.Conv_IntToDouble` _y) 1.524) _returnvalue))
      (`SceneComponent.SetWorldScale3D` (`self.CornerR`) (`KismetMathLibrary.MakeVector` (* (`KismetMathLibrary.Conv_IntToDouble` _x) 1.524) _returnvalue_2 _returnvalue))
      (`SceneComponent.SetWorldScale3D` (`self.CornerTR`) (`KismetMathLibrary.MakeVector` _returnvalue_3 _returnvalue_2 _returnvalue)))))

(fn `UserConstructionScript`)