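; World grid cell that tracks which interactables and pawns occupy it or block its space.
; Sphere overlaps sort actors by type message, registering those centered in the cell's grid space and counting others as blocking space.
; End overlaps remove pawns by ID or release blocking space, but leave centered objects registered.
; Each change refreshes a mesh showing occupancy when the parent grid's collision display is on.
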(event `self.Sphere.OnComponentBeginOverlap`
  (params (OverlappedComponent :type "PrimitiveComponent Object Reference") (OtherActor :type "Actor Object Reference") (OtherComp :type "PrimitiveComponent Object Reference") (OtherBodyIndex :type Integer) (bFromSweep :type Boolean) (SweepResult :type "HitResult Structure (by ref)"))
  (bind _returnvalue (`self.ComparePositionGridSpace` OtherActor))
  (`/Engine/EditorBlueprintResources/StandardMacros.IsValid` OtherActor
    (:`Is Valid`
      (bind _returnvalue_2 (message `GridEntity.GetType` OtherActor))
      (switch `GRID_OBJECT_TYPE` _returnvalue_2
        (:`INTERACTABLE`
          (`self.AddNewObject` OtherActor _returnvalue_2 _returnvalue)
          (`self.UpdateCollision`))
        (:`PAWN`
          (`self.AddNewPawn` OtherActor _returnvalue)
          (`self.UpdateCollision`))))))

(event `self.Sphere.OnComponentEndOverlap`
  (params (OverlappedComponent :type "PrimitiveComponent Object Reference") (OtherActor :type "Actor Object Reference") (OtherComp :type "PrimitiveComponent Object Reference") (OtherBodyIndex :type Integer))
  (bind _returnvalue (`self.ComparePositionGridSpace` OtherActor))
  (`/Engine/EditorBlueprintResources/StandardMacros.IsValid` OtherActor
    (:`Is Valid`
      (bind _returnvalue_2 (message `GridEntity.GetType` OtherActor))
      (switch `GRID_OBJECT_TYPE` _returnvalue_2
        (:`INTERACTABLE`
          (`self.RemoveCurrentObject` _returnvalue)
          (`self.UpdateCollision`))
        (:`PAWN`
          (`self.RemoveCurrentPawn` OtherActor _returnvalue)
          (`self.UpdateCollision`))))))

(fn `AddNewObject`
  (params (Object :type "Actor Object Reference") (Type :type "GRID_OBJECT_TYPE Enum" :default "NONE") (CenterOfMassOverlaps :type Boolean))
  (if CenterOfMassOverlaps
    (`self.AddObject` Type Object)
    (else
      (`self.AddBlockingSpace`))))

(fn `AddNewPawn`
  (params (Pawn :type "Actor Object Reference") (`Center Of Mass Overlaps` :type Boolean))
  (if `Center Of Mass Overlaps`
    (bind _returnvalue (`self.AddPawn` Pawn))
    (`KismetSystemLibrary.PrintString` (`KismetStringLibrary.Conv_BoolToString` _returnvalue))
    (else
      (`self.AddBlockingSpace`))))

(fn `RemoveCurrentObject`
  (params (CenterOfMassOverlaps :type Boolean))
  (if (not CenterOfMassOverlaps)
    (`self.RemoveBlockingSpace`)))

(fn `RemoveCurrentPawn`
  (params (Pawn :type "Actor Object Reference") (CenterOfMassOverlaps :type Boolean))
  (if CenterOfMassOverlaps
    (bind _asbp_map_pawn (cast `/Game/Blueprints/Characters/BP_MapPawn` Pawn))
    (`self.RemovePawn` (`MapPawn.GetPawnID` _asbp_map_pawn))
    (else
      (`self.RemoveBlockingSpace`))))

(fn `UpdateCollision`
  (bind _parentgrid (`self.ParentGrid`))
  (`/Engine/EditorBlueprintResources/StandardMacros.IsValid` _parentgrid
    (:`Is Valid`
      (if (`WorldGrid.bShowCollisions` _parentgrid)
        (`SceneComponent.SetVisibility` (`self.StaticMesh`) (`self.IsOcupied`) false)))))

(fn `UserConstructionScript`)