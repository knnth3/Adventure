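; Adventure game instance that owns the pause menu and handles the move into the multiplayer lobby.
; On Init it creates the pause menu widget for the first player controller and stores it, with functions to query and toggle its active state.
; The multiplayer load event opens the lobby level as a listen server.
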(event `self.ReceiveInit`
  (bind _returnvalue (`|CreateWidget` "/Game/Blueprints/UI/Multiplayer/PauseMenu.PauseMenu_C" (`GameplayStatics.GetPlayerController` 0)))
  (set `self.PauseMenu` _returnvalue))

(event `self.OnLoadMultiplayerMap`
  (`GameplayStatics.OpenLevel` "Level_Lobby" true "?listen"))

(fn `IsPauseMenuActive`
  (returns (Value :type Boolean))
  (bind _pausemenu (`self.PauseMenu`))
  (`/Engine/EditorBlueprintResources/StandardMacros.IsValid` _pausemenu
    (:`Is Valid`
      (return (`W_PauseMenu.IsActive` _pausemenu)))
    (:`Is Not Valid`
      (return false))))

(fn `TogglePauseMenu`
  (bind _pausemenu (`self.PauseMenu`))
  (if (`W_PauseMenu.IsActive` _pausemenu)
    (`W_PauseMenu.Deactivate` _pausemenu)
    (else
      (`W_PauseMenu.Activate` _pausemenu))))