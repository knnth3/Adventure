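; BP_MapPawn is a clickable, space-blocking pawn on a grid map that reports clicks to the player controller and highlights on hover.
; It starts with two equipped items and a one-handed weapon type, unequipping on destruction.
; Attacks go through the attack component, while Tick rotates a turn vector toward the desired facing.
; Status changes drive particle effects, with the frozen status pausing mesh animation via its global rate scale.
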(event `self.ReceiveBeginPlay`
  (bind _bp_inventorycomponent (`self.BP_InventoryComponent`))
  (`|ExecutionSequence`
    (:`then_0`
      (`InventoryComponent.AddObject` _bp_inventorycomponent 8 1)
      (`InventoryComponent.AddObject` _bp_inventorycomponent 7 1)
      (`InventoryComponent.EquipObject` _bp_inventorycomponent 7 true)
      (`InventoryComponent.EquipObject` _bp_inventorycomponent 8 false)
      (`self.ServerOnly_SetEquipedWeaponType` "STAFF_1H"))
    (:`then_1`
      ;[1 1 1] Add components that can be highlighted when mouse over event or selection
      (`HighlightComponent.AddHighlightableComponents` (`self.Highlight`) (`|MakeArray` (`self.Mesh`) (`self.PawnHeadComponent`) :!type "PrimitiveComponent Object Reference")))))

(event `self.ReceiveActorBeginCursorOver`
  ;[1 1 1] Add components that can be highlighted when mouse over event or selection
  (`HighlightComponent.HighlightObjects` (`self.Highlight`)))

(event `self.ReceiveActorEndCursorOver`
  ;[1 1 1] Add components that can be highlighted when mouse over event or selection
  (`HighlightComponent.DimObjects` (`self.Highlight`)))

(event `self.ReceiveTick`
  (params (DeltaSeconds :type "Float (single-precision)"))
  (bind (_returnvalue_x _returnvalue_y) (`KismetMathLibrary.BreakVector` (`self.ServerOnly_GetDesiredForwardVector`)))
  (`SceneComponent.K2_SetWorldRotation` (`self.TurnVector`) (`KismetMathLibrary.MakeRotator` 0.0 0.0 (`KismetMathLibrary.DegAtan2` _returnvalue_y _returnvalue_x)) false false))

(event `self.ReceiveActorOnClicked`
  (params (ButtonPressed :type "Key Structure"))
  (message `/Game/Blueprints/Interfaces/BP_SelectorInterface.OnPawnSelected` (`GameplayStatics.GetPlayerController` 0) self))

(event `self.OnAttackInitiated`
  (params (AttackIndex :type Integer) (TargetLocation :type "Vector Structure (by ref)"))
  (`/Game/Blueprints/Components/BP_AttackComponent.Attack` (`self.BP_AttackComponent`) TargetLocation)
  (`self.ServerOnly_SetTargetLocation` TargetLocation)
  (set `self.bIsAttacking` true))

(event `self.BP_AttackComponent.Event OnAttackEnd`
  (set `self.bIsAttacking` false))

(event `self.OnStatusChanged`
  (params (StatusID :type Integer))
  (bind _bp_goodparticlestatus (`self.BP_GoodParticleStatus`))
  (bind _mesh (`self.Mesh`))
  (bind _returnvalue (cast `/Game/Plugins/GoodParticleStatus/Blueprint/Enum/Enum_GoodParticleStatus` (`KismetSystemLibrary.MakeLiteralByte` (`KismetMathLibrary.Conv_IntToByte` StatusID))))
  (bind _returnvalue_2 (`|EnumEquality` _returnvalue "NewEnumerator11"))
  (set `/Game/Plugins/GoodParticleStatus/Blueprint/BP_GoodParticleStatus.Effects Style` "NewEnumerator2" _bp_goodparticlestatus)
  (`/Game/Plugins/GoodParticleStatus/Blueprint/BP_GoodParticleStatus.GoodParticleStatus Update` _bp_goodparticlestatus)
  (set `/Game/Plugins/GoodParticleStatus/Blueprint/BP_GoodParticleStatus.Effects Style` _returnvalue _bp_goodparticlestatus)
  (`/Game/Plugins/GoodParticleStatus/Blueprint/BP_GoodParticleStatus.GoodParticleStatus Update` _bp_goodparticlestatus)
  (if (!= (`self.bIsFrozen`) _returnvalue_2)
    (bind _output_get (set `self.bIsFrozen` _returnvalue_2))
    (if _output_get
      (set `SkeletalMeshComponent.GlobalAnimRateScale` 0.0 _mesh)
      (else
        (set `SkeletalMeshComponent.GlobalAnimRateScale` 1.0 _mesh)))))

(event `self.ReceiveDestroyed`
  (bind _bp_inventorycomponent (`self.BP_InventoryComponent`))
  (`InventoryComponent.UnequipObject` _bp_inventorycomponent true)
  (`InventoryComponent.UnequipObject` _bp_inventorycomponent false))

(fn `Deselect`
  (`HighlightComponent.DimObjects` (`self.Highlight`)))

(fn `GetLocationGridSpace`
  (returns (ReturnValue :type "GridCoordinate Structure"))
  (return (`GridFunctions.WorldToGridLocation` (`self.K2_GetActorLocation`))))

(fn `GetLocationWorldSpace`
  (returns (ReturnValue :type "Vector Structure"))
  (return (`self.K2_GetActorLocation`)))

(fn `GetObjectID`
  (returns (ReturnValue :type Integer))
  (return (`self.GetPawnID`)))

(fn `GetType`
  (returns (ReturnValue :type "GRID_OBJECT_TYPE Enum"))
  (return "PAWN"))

(fn `IsBlockingSpace`
  (returns (ReturnValue :type Boolean))
  (return true))

(fn `Select`)

(fn `UserConstructionScript`)