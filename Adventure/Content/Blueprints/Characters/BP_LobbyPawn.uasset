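; BP_LobbyPawn is a lobby character pawn with a swappable head and an overhead name label.
; On BeginPlay it spawns a BP_MapPawn_Head actor attached to the skeletal mesh's head socket, and clients also create the client HUD.
; CursorSelect cycles through boy head meshes, advancing the wrapping index only when SetMesh succeeds.
; SetOverheadText sets the Name variable, whose OnRep updates the TextRender.
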(event `self.ReceiveBeginPlay`
  (bind _returnvalue (`|SpawnActorFromClass` "/Game/Blueprints/Characters/BP_MapPawn_Head.BP_MapPawn_Head_C" (`KismetMathLibrary.MakeTransform` (0.0 0.0 0.0)) "AlwaysSpawn" "OverrideRootScale" null null))
  (bind _output_get (set `self.HeadActor` _returnvalue))
  (`self.K2_AttachToComponent` _output_get (`self.SkeletalMesh`) "biped_mr_NA_Head" "SnapToTarget" "SnapToTarget" "KeepWorld" true)
  (`/Game/Blueprints/Public/PublicMacros.Switch On Server`
    (:`Client`
      (bind _returnvalue_2 (`|CreateWidget` "/Game/Blueprints/UI/Lobby/BP_Client_HUD.BP_Client_HUD_C" (`GameplayStatics.GetPlayerController` 0)))
      (`UserWidget.AddToViewport` _returnvalue_2 0))))

(event `InputAction|CursorSelect`
  (params (Key :type "Key Structure"))
  (bind _headactor (`self.HeadActor`))
  (bind _index (`self.index`))
  (:`Pressed`
    (`/Engine/EditorBlueprintResources/StandardMacros.IsValid` _headactor
      (:`Is Valid`
        (bind _success (`/Game/Blueprints/Characters/BP_MapPawn_Head.SetMesh` _headactor _index true))
        (if _success
          (set `self.index` (mod (+ _index 1) 57)))))))

(fn `OnRep_Name`
  (`TextRenderComponent.K2_SetText` (`self.TextRender`) (`self.Name`)))

(fn `SetOverheadText`
  (params (Name :type Text))
  (set `self.Name` Name))

(fn `UserConstructionScript`)