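; BP_PaintCursor is a preview cursor actor for placing meshes as blocking objects on the world grid.
; It caches the first BP_WorldGrid on BeginPlay and exposes functions to set its mesh and index, toggle visibility, and move it, optionally snapped to grid cells.
; Placement passes the stored mesh index as a class index, with a transform, to the grid's ServerOnlyAddBlockingObject.
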(event `self.ReceiveBeginPlay`
  (bind _outactors (`GameplayStatics.GetAllActorsOfClass` "/Game/Blueprints/Grid/BP_WorldGrid.BP_WorldGrid_C"))
  (set `self.WorldGrid` (`|GetArrayItem` _outactors)))

(fn `AddMeshToGrid`
  (params (Transform :type "Transform Structure"))
  (bind _worldgrid (`self.WorldGrid`))
  (`/Engine/EditorBlueprintResources/StandardMacros.IsValid` _worldgrid
    (:`Is Valid`
      (`WorldGrid.ServerOnly_AddBlockingObject` _worldgrid (`self.MeshIndex`) Transform))))

(fn `DisplayCursor`
  (params (Visibility :type Boolean))
  (`SceneComponent.SetVisibility` (`self.StaticMesh`) Visibility false))

(fn `IsVisible`
  (returns (Value :type Boolean))
  (return (`SceneComponent.IsVisible` (`self.StaticMesh`))))

(fn `SetCursorLocation`
  (params (Location :type "Vector Structure"))
  (if (`self.SnapMovement`)
    (`self.K2_SetActorLocation` (`GridFunctions.GridToWorldLocation` (`GridFunctions.WorldToGridLocation` Location)))
    (else
      (`self.K2_SetActorLocation` Location))))

(fn `SetStaticMesh`
  (params (MeshIndex :type Byte) (Mesh :type "StaticMesh Object Reference"))
  (set `self.MeshIndex` MeshIndex)
  (`StaticMeshComponent.SetStaticMesh` (`self.StaticMesh`) Mesh))

(fn `SnapMovementToGrid`
  (params (Value :type Boolean))
  (set `self.SnapMovement` Value))

(fn `UserConstructionScript`)