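; BP_SpectatorMapPawn is a spectator pawn that pans and zooms a map view for the adventure editor's player controller.
; On BeginPlay it caches the BP_PC_Adventure_Editor controller, whose MenuActive check blocks all movement input while a menu is open.
; Look axes offset the actor along world X and Y without sweeping, and Zoom changes the camera boom's arm length.
; All three scale with Speed and frame delta time.
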(event `self.ReceiveBeginPlay`
  (bind _asbp_pc_adventure_editor (cast `/Game/Blueprints/PlayerControllers/BP_PC_Adventure_Editor` (`GameplayStatics.GetPlayerController` 0)))
  (set `self.MyController` _asbp_pc_adventure_editor))

(event `InputAxis|LookUp-Down`
  (params (AxisValue :type "Float (single-precision)"))
  (if (not (`/Game/Blueprints/PlayerControllers/BP_PC_Adventure_Editor.MenuActive` (`self.MyController`)))
    (if (!= AxisValue 0.0)
      (`self.K2_AddActorWorldOffset` (* (1.0 0.0 0.0) (* AxisValue (`GameplayStatics.GetWorldDeltaSeconds`) (`self.Speed`) 100.0))))))

(event `InputAxis|LookLeft-Right`
  (params (AxisValue :type "Float (single-precision)"))
  (if (not (`/Game/Blueprints/PlayerControllers/BP_PC_Adventure_Editor.MenuActive` (`self.MyController`)))
    (if (!= AxisValue 0.0)
      (`self.K2_AddActorWorldOffset` (* (0.0 1.0 0.0) (* AxisValue (`GameplayStatics.GetWorldDeltaSeconds`) (`self.Speed`) 100.0))))))

(event `InputAxis|Zoom`
  (params (AxisValue :type "Float (single-precision)"))
  (bind _cameraboom (`self.CameraBoom`))
  (if (not (`/Game/Blueprints/PlayerControllers/BP_PC_Adventure_Editor.MenuActive` (`self.MyController`)))
    (if (!= AxisValue 0.0)
      (set `SpringArmComponent.TargetArmLength` (+ (`SpringArmComponent.TargetArmLength` _cameraboom) (* (`self.Speed`) (`GameplayStatics.GetWorldDeltaSeconds`) AxisValue -300.0)) _cameraboom))))

(fn `UserConstructionScript`)