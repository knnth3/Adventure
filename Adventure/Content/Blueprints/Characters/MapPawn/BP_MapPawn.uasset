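; BP_MapPawn is a map pawn that handles click-to-move on a grid and an orbiting, zoomable camera.
; CursorSelect traces under the mouse, snaps the hit to the grid via a world-to-grid-to-world conversion, and passes it to SetDestination.
; Axis inputs yaw and pitch the CameraBoom or change its arm length, scaled by frame time and CameraSettings speeds, with pitch and zoom clamped to configured limits.
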(event `self.ReceiveTick`
  (params (DeltaSeconds :type "Float (single-precision)")))

(event `InputAction|CursorSelect`
  (params (Key :type "Key Structure"))
  (bind (_world_location _success) (`/Game/Blueprints/Public/PublicFunctions.GetMouseCoordinates3D` "TraceTypeQuery3"))
  (:`Pressed`
    (if _success
      (`self.SetDestination` (`GridFunctions.GridToWorldLocation` (`GridFunctions.WorldToGridLocation` _world_location))))))

(event `InputAxis|LookUp-Down`
  (params (AxisValue :type "Float (single-precision)"))
  (`self.RotateUpDown` AxisValue (`GameplayStatics.GetWorldDeltaSeconds`)))

(event `InputAxis|LookLeft-Right`
  (params (AxisValue :type "Float (single-precision)"))
  (`self.RotateLeftRight` AxisValue (`GameplayStatics.GetWorldDeltaSeconds`)))

(event `InputAxis|Zoom`
  (params (AxisValue :type "Float (single-precision)"))
  (`self.Zoom` AxisValue (`GameplayStatics.GetWorldDeltaSeconds`)))

(fn `RotateLeftRight`
  (params (`Axis Value` :type "Float (double-precision)") (`Delta Time` :type "Float (double-precision)"))
  (bind _cameraboom (`self.CameraBoom`))
  (bind (_returnvalue_roll _returnvalue_pitch _returnvalue_yaw) (`KismetMathLibrary.BreakRotator` (`SceneComponent.K2_GetComponentRotation` _cameraboom)))
  (if (!= `Axis Value` 0.0)
    (`SceneComponent.K2_SetWorldRotation` _cameraboom (`KismetMathLibrary.MakeRotator` _returnvalue_roll _returnvalue_pitch (- _returnvalue_yaw (* `Axis Value` `Delta Time` (`.AngularVelocity` (break `CameraSettings` (`self.CameraSettings`)))))) false false)))

(fn `RotateUpDown`
  (params (`Axis Value` :type "Float (double-precision)") (`Delta Time` :type "Float (double-precision)"))
  (bind _cameraboom (`self.CameraBoom`))
  (bind (_angularvelocity _zoomspeed _maxuprotation _maxdownrotation) (break `CameraSettings` (`self.CameraSettings`)))
  (bind (_returnvalue_roll _returnvalue_pitch _returnvalue_yaw) (`KismetMathLibrary.BreakRotator` (`SceneComponent.K2_GetComponentRotation` _cameraboom)))
  (if (!= `Axis Value` 0.0)
    (`SceneComponent.K2_SetWorldRotation` _cameraboom (`KismetMathLibrary.MakeRotator` _returnvalue_roll (`KismetMathLibrary.ClampAngle` (- _returnvalue_pitch (* `Axis Value` `Delta Time` _angularvelocity)) _maxuprotation _maxdownrotation) _returnvalue_yaw) false false)))

(fn `UserConstructionScript`)

(fn `Zoom`
  (params (`Axis Value` :type "Float (double-precision)") (`Delta Time` :type "Float (double-precision)"))
  (bind _cameraboom (`self.CameraBoom`))
  (bind (_angularvelocity _zoomspeed _maxuprotation _maxdownrotation _maxinzoom _maxoutzoom) (break `CameraSettings` (`self.CameraSettings`)))
  (if (!= `Axis Value` 0.0)
    (set `SpringArmComponent.TargetArmLength` (`KismetMathLibrary.FClamp` (+ (`SpringArmComponent.TargetArmLength` _cameraboom) (* `Axis Value` `Delta Time` _zoomspeed -1.0)) _maxinzoom _maxoutzoom) _cameraboom)))