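; SelectCursor is a cursor actor that hovers above a given location, bobbing vertically while facing the camera.
; While visible, Tick advances a wrapped angle to drive a cosine float above BaseHeight and yaws the actor toward the player camera in the horizontal plane.
; Position updates teleport it in X/Y and reset BaseHeight slightly above the location.
; Visibility changes toggle the root and its children.
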(event `self.ReceiveBeginPlay`)

(event `self.ReceiveTick`
  (params (DeltaSeconds :type "Float (single-precision)"))
  (bind (_returnvalue_x _returnvalue_y) (`KismetMathLibrary.BreakVector` (`self.K2_GetActorLocation`)))
  (bind (_returnvalue_x_2 _returnvalue_y_2) (`KismetMathLibrary.BreakVector` (`PlayerCameraManager.GetCameraLocation` (`GameplayStatics.GetPlayerCameraManager` 0))))
  (bind (_returnvalue_x_3 _returnvalue_y_3) (`KismetMathLibrary.BreakVector` (- (`KismetMathLibrary.MakeVector` _returnvalue_x_2 _returnvalue_y_2) (`KismetMathLibrary.MakeVector` _returnvalue_x _returnvalue_y))))
  (if (`SceneComponent.IsVisible` (`self.DefaultSceneRoot`))
    (bind _output_get (set `self.animTime` (mod (+ (* DeltaSeconds (`self.angularVelocity`)) (`self.animTime`)) 360.0)))
    (`self.K2_SetActorLocation` (`KismetMathLibrary.MakeVector` _returnvalue_x _returnvalue_y (+ (* (`KismetMathLibrary.DegCos` _output_get) (`self.float radius`)) (`self.BaseHeight`) (`self.float radius`))))
    (`self.K2_SetActorRotation` (`KismetMathLibrary.MakeRotator` 0.0 0.0 (`KismetMathLibrary.DegAtan2` _returnvalue_y_3 _returnvalue_x_3)))))

(event `OnPositionUpdate`
  (params (Location :type "Vector Structure"))
  (`self.SetBaseLocation` Location))

(event `OnVisibilityChanged`
  (params (value :type Boolean))
  (bind _defaultsceneroot (`self.DefaultSceneRoot`))
  (if (!= (`SceneComponent.IsVisible` _defaultsceneroot) value)
    (`SceneComponent.SetVisibility` _defaultsceneroot value true)))

(fn `SetBaseLocation`
  (params (Location :type "Vector Structure"))
  (bind (_returnvalue_x _returnvalue_y _returnvalue_z) (`KismetMathLibrary.BreakVector` (`self.K2_GetActorLocation`)))
  (set `self.BaseHeight` (+ Location_Z 15.0))
  (`self.K2_SetActorLocation` (`KismetMathLibrary.MakeVector` Location_X Location_Y _returnvalue_z) false true))

(fn `UserConstructionScript`)