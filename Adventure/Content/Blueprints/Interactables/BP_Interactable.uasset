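; Interactable actor for the adventure editor that highlights under the cursor and reports its selection when clicked.
; A Highlight component, given the Visual component at BeginPlay, highlights on hover only in editor mode 2 and dims on cursor exit.
; The GetEditorMode macro branches on the selected mode of BP_PC_Adventure_Editor.
; Clicks send the actor to the player controller in any mode, and GetType identifies it as INTERACTABLE.
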(event `self.ReceiveBeginPlay`
  (`HighlightComponent.AddHighlightableComponents` (`self.Highlight`) (`|MakeArray` (`self.Visual`) :!type "PrimitiveComponent Object Reference")))

(event `self.ReceiveActorBeginCursorOver`
  (`self.GetEditorMode`
    (:`2`
      (`HighlightComponent.HighlightObjects` (`self.Highlight`)))))

(event `self.ReceiveActorEndCursorOver`
  (`self.GetEditorMode`
    (:`0`
      _)
    (:`1`
      _)
    (:`2`
      _)
    (:`Default`
      _))
  (`HighlightComponent.DimObjects` (`self.Highlight`)))

(event `self.ReceiveActorOnClicked`
  (params (ButtonPressed :type "Key Structure"))
  (message `/Game/Blueprints/Interfaces/BP_SelectorInterface.OnObjectSelected` (`GameplayStatics.GetPlayerController` 0) self))

(fn `GetType`
  (returns (ReturnValue :type "GRID_OBJECT_TYPE Enum"))
  (return "INTERACTABLE"))

(fn `UserConstructionScript`)