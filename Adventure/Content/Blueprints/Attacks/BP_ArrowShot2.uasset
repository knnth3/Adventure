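; Arrow shot attack actor that plays a launch effect and fires a BP_ArrowProj2 projectile toward a destination.
; On initialization it raises the destination to match its own raised spawn height, turns to face it, activates the AttackAnim effect and spawns the projectile with direction, speed and maximum distance.
; It then nudges itself forward along the shot direction and destroys itself when the effect finishes.
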(event `self.ReceiveBeginPlay`
  (`self.K2_AddActorWorldOffset` (0.0 0.0 76.199997)))

(event `self.OnInitialized`
  (bind _returnvalue (`self.K2_GetActorLocation`))
  (bind (_destination_x _destination_y _destination_z) (`KismetMathLibrary.BreakVector` (`self.Destination`)))
  (bind _output_get (set `self.Destination` (`KismetMathLibrary.MakeVector` _destination_x _destination_y (+ _destination_z 76.199997))))
  (bind _output_get_2 (set `self.ForwardVector` (`KismetMathLibrary.Normal` (- _output_get _returnvalue))))
  (bind _returnvalue_2 (`KismetMathLibrary.FindLookAtRotation` (`KismetMathLibrary.MakeVector` 0.0) _output_get_2))
  (`self.K2_SetActorRotation` _returnvalue_2)
  (`ActorComponent.Activate` (`self.AttackAnim`) true)
  (`|SpawnActorFromClass` "/Game/Blueprints/Attacks/BP_ArrowProj2.BP_ArrowProj2_C" (`KismetMathLibrary.MakeTransform` _returnvalue _returnvalue_2) "AlwaysSpawn" "OverrideRootScale" (`self.GetOwner`) (`self.ProjSpeed`) _output_get_2 (`self.MaxDistance`) null)
  (`self.K2_AddActorWorldOffset` (* (`self.ForwardVector`) 150.0)))

(event `self.AttackAnim.OnSystemFinished`
  (params (PSystem :type "ParticleSystemComponent Object Reference"))
  (`self.K2_DestroyActor`))

(fn `UserConstructionScript`)