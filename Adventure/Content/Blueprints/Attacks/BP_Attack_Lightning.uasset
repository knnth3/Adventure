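; BP_Attack_Lightning is a lightning attack actor that moves to the target location and anchors its StartLocation component at the caster's location.
; On BeginPlay it plays audio, waits, briefly shows the hit and emitter particles, and starts a Duration timer.
; When the timer fires, it destroys itself and notifies a valid Parent that the attack ended.
; The construction script feeds the actor into an emitter particle instance parameter.
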(event `self.ReceiveBeginPlay`
  (`self.K2_SetActorLocation` (`self.TargetLocation`))
  (`SceneComponent.K2_SetWorldLocation` (`self.StartLocation`) (`self.CasterLocation`) false false)
  (`AudioComponent.Play` (`self.Audio`) 0.0)
  (`KismetSystemLibrary.Delay` 1.55)
  (`SceneComponent.SetVisibility` (`self.HitParticles`) true false)
  (`SceneComponent.SetVisibility` (`self.EmitterParticles`) true false)
  (`KismetSystemLibrary.K2_SetTimerDelegate` (delegate `Event BeginDestroy`) (`self.Duration`))
  (`KismetSystemLibrary.Delay` 0.4)
  (`SceneComponent.SetVisibility` (`self.HitParticles`) false false)
  (`SceneComponent.SetVisibility` (`self.EmitterParticles`) false false))

(event `Event BeginDestroy`
  (bind _parent (`self.Parent`))
  (`self.K2_DestroyActor`)
  (`/Engine/EditorBlueprintResources/StandardMacros.IsValid` _parent
    (:`Is Valid`
      (`/Game/Blueprints/Components/BP_AttackComponent.Event OnAttackEnd` _parent))))

(fn `UserConstructionScript`
  (set `ParticleSystemComponent.InstanceParameters` (`|MakeArray` (make `ParticleSysParam` "2" "PSPT_Vector" 0.0 0.0 (0.0 0.0 0.0) (0.0 0.0 0.0) (struct) self)) (`self.EmitterParticles`)))