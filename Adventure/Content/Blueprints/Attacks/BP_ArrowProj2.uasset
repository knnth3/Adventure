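; BP_ArrowProj2 is an arrow projectile attack that damages the first living map pawns it touches, ignoring its owner.
; Tick moves it along its forward vector without sweeping until it travels MaxDistance or its Impact effect is active.
; A sphere overlap deactivates the Projectile effect, activates Impact, nudges the arrow forward and applies fixed damage through the pawn's interaction interface.
; The actor destroys itself when the Impact system finishes.
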(event `self.ReceiveTick`
  (params (DeltaSeconds :type "Float (single-precision)"))
  (bind _returnvalue (* DeltaSeconds (`self.ProjSpeed`)))
  (if (`ActorComponent.IsActive` (`self.Impact`))
    (`/Engine/EditorBlueprintResources/StandardMacros.DoOnce` (`self.bProjIsDeactivated`)
      (:`Completed`
        (`ActorComponent.Deactivate` (`self.Projectile`))))
    (else
      (`self.K2_AddActorWorldOffset` (* (`self.ForwardVector`) _returnvalue))
      (bind _output_get (set `self.TotalDistance` (+ _returnvalue (`self.TotalDistance`))))
      (if (>= _output_get (`self.MaxDistance`))
        (`ActorComponent.Activate` (`self.Impact`) true)))))

(event `self.Impact.OnSystemFinished`
  (params (PSystem :type "ParticleSystemComponent Object Reference"))
  (`self.K2_DestroyActor`))

(event `self.Sphere.OnComponentBeginOverlap`
  (params (OverlappedComponent :type "PrimitiveComponent Object Reference") (OtherActor :type "Actor Object Reference") (OtherComp :type "PrimitiveComponent Object Reference") (OtherBodyIndex :type Integer) (bFromSweep :type Boolean) (SweepResult :type "HitResult Structure (by ref)"))
  (if (!= OtherActor (`self.GetOwner`))
    (bind _asbp_map_pawn (cast `/Game/Blueprints/Actors/BP_MapPawn` OtherActor))
    (if (`|EnumInequality` (`StatisticsComponent.GetCurrentAction` (`MapPawn.GetStats` _asbp_map_pawn)) "DEAD")
      (set `self.bProjIsDeactivated` true)
      (`ActorComponent.Deactivate` (`self.Projectile`))
      (`ActorComponent.Activate` (`self.Impact`) true)
      (`self.K2_AddActorWorldOffset` (* (`self.ForwardVector`) 38.099998))
      (`InteractionInterfaceComponent.TakeDamage` (`MapPawn.GetInteractionInterface` _asbp_map_pawn) 11 (`self.K2_GetActorLocation` (`self.GetOwner` _asbp_map_pawn))))))

(fn `UserConstructionScript`)