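; BP_MeleeAttack is a short-lived melee hitbox actor that damages map pawns it touches.
; On initialization it moves its sphere to the destination, then on overlap with a BP_MapPawn other than its owner it deals 1 damage through that pawn's interaction interface, passing the owner's location as the attacker position.
; It destroys itself after that hit or once it has lived for about one second, tracked in Tick.
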(event `self.OnInitialized`
  (`SceneComponent.K2_SetWorldLocation` (`self.Sphere`) (`self.Destination`) false false))

(event `self.Sphere.OnComponentBeginOverlap`
  (params (OverlappedComponent :type "PrimitiveComponent Object Reference") (OtherActor :type "Actor Object Reference") (OtherComp :type "PrimitiveComponent Object Reference") (OtherBodyIndex :type Integer) (bFromSweep :type Boolean) (SweepResult :type "HitResult Structure (by ref)"))
  (bind _returnvalue (`self.GetOwner`))
  (if (!= _returnvalue OtherActor)
    (bind _asbp_map_pawn (cast `/Game/Blueprints/Actors/BP_MapPawn` OtherActor))
    (`InteractionInterfaceComponent.TakeDamage` (`MapPawn.GetInteractionInterface` _asbp_map_pawn) 1 (`self.K2_GetActorLocation` _returnvalue))
    (`self.K2_DestroyActor`)))

(event `self.ReceiveTick`
  (params (DeltaSeconds :type "Float (single-precision)"))
  (bind _output_get (set `self.timeAlive` (+ DeltaSeconds (`self.timeAlive`))))
  (if (> _output_get 1.0)
    (`self.K2_DestroyActor`)))

(fn `UserConstructionScript`)