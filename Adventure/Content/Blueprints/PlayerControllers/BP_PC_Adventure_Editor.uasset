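; Player controller for the Adventure map editor, letting the player place and delete grid objects with the cursor.
; BeginPlay builds the GameBuilderUI from game mode map data and respawns saved objects for existing maps.
; Clicks outside menus are traced, snapped to grid and handled by UI mode: draw interactable, set spawn or delete.
; Successful world requests are then logged to the UI as edit events; pausing goes through the game instance.
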(event `self.ReceiveBeginPlay`
  (`|ExecutionSequence`
    (:`then_0`
      ;[1 1 1] Create the Editor UI
      (bind _asbp_gm_game_builder (cast `/Game/Blueprints/GameModes/BP_GM_GameBuilder` (`GameplayStatics.GetGameMode`)))
      (bind _returnvalue (`GM_GameBuilder.IsNewMap` _asbp_gm_game_builder))
      (bind _returnvalue_2 (`|CreateWidget` "/Game/Blueprints/UI/GameBuilder/GameBuilderUI.GameBuilderUI_C" null (`KismetStringLibrary.Conv_NameToString` (`GM_GameBuilder.GetMapName` _asbp_gm_game_builder)) (`GM_GameBuilder.GetMapSize` _asbp_gm_game_builder) _returnvalue))
      (bind _output_get (set `self.UI` _returnvalue_2))
      (`WidgetBlueprintLibrary.SetInputMode_GameAndUIEx` self _output_get "DoNotLock" false)
      (`UserWidget.AddToViewport` _output_get 0)
      (if (not _returnvalue)
        (`self.SpawnObjectsFromList` (`W_GameBuilderUI.GetAllObjects` _returnvalue_2))))
    (:`then_1`
      (bind _asbp_gi_adventure (cast `/Game/Blueprints/GameInstance/BP_GI_Adventure` (`GameplayStatics.GetGameInstance`)))
      (set `self.GameInstance` _asbp_gi_adventure))))

(event `InputAction|Pause`
  (params (Key :type "Key Structure"))
  (bind _gameinstance (`self.GameInstance`))
  (:`Pressed`
    (`/Engine/EditorBlueprintResources/StandardMacros.IsValid` _gameinstance
      (:`Is Valid`
        (`/Game/Blueprints/GameInstance/BP_GI_Adventure.TogglePauseMenu` _gameinstance)))))

(event `InputAction|CursorSelect`
  (params (Key :type "Key Structure"))
  (bind (_world_location _success) (`/Game/Blueprints/Public/PublicFunctions.GetMouseCoordinates3D` "TraceTypeQuery3"))
  (bind _ui (`self.UI`))
  (bind _returnvalue (`GridFunctions.WorldToGridLocation` _world_location))
  (bind _selectedmodelindex (`/Game/Blueprints/UI/GameBuilder/GameBuilderUI.SelectedModelIndex` _ui))
  (bind _selectedmode (`/Game/Blueprints/UI/GameBuilder/GameBuilderUI.SelectedMode` _ui))
  (bind (_type_modelindex _type_location _type_type) (break `GAMEBUILDER_OBJECT` (`W_GameBuilderUI.GetObjecteByCoordinate` _ui _returnvalue)))
  (:`Pressed`
    (if (`self.MenuActive`)
      _
      (elif _success
        (`KismetSystemLibrary.PrintString` (`KismetStringLibrary.Conv_IntToString` _selectedmode))
        (switch `int` _selectedmode
          (:`0`
            ;[1 1 1] Draw mode
            (bind _returnvalue_2 (`self.RequestSpawnInteractible` _selectedmodelindex _returnvalue))
            (if _returnvalue_2
              (bind _returnvalue_3 (`W_GameBuilderUI.SubmitEditEvent` _ui "INTERACTABLE" (make `GAMEBUILDER_EDIT_EVENT` _selectedmodelindex "CREATE" (struct) _returnvalue)))
              (if _returnvalue_3
                (`KismetSystemLibrary.PrintString` "Createtion Log Success!")
                (else
                  (`KismetSystemLibrary.PrintString` "Createtion Log Failed!")))
              (else
                (`KismetSystemLibrary.PrintString` "Spawn Interactible Failed!"))))
          (:`1`
            ;[1 1 1] Spawn creation mode
            (bind _returnvalue_4 (`self.RequestSetSpawnLocation` _selectedmodelindex _returnvalue))
            (if _returnvalue_4
              (bind _returnvalue_5 (`W_GameBuilderUI.SubmitEditEvent` _ui "SPAWN" (make `GAMEBUILDER_EDIT_EVENT` _selectedmodelindex "CREATE" (struct) _returnvalue)))
              (if _returnvalue_5
                (`KismetSystemLibrary.PrintString` "Spawn Location Added!")
                (else
                  (`KismetSystemLibrary.PrintString` "Spawn Location failed to add.")))
              (else
                (`KismetSystemLibrary.PrintString` "Could not  create the given spawn location."))))
          (:`2`
            ;[1 1 1] Delete mode
            (if (`|EnumInequality` _type_type "ANY")
              (bind _returnvalue_6 (`self.RequestDeleteObject` _type_type _returnvalue))
              (if _returnvalue_6
                (bind _returnvalue_7 (`W_GameBuilderUI.SubmitEditEvent` _ui _type_type (make `GAMEBUILDER_EDIT_EVENT` 0 "DELETE" _returnvalue)))
                (if _returnvalue_7
                  (`KismetSystemLibrary.PrintString` "Object Delete Success")
                  (else
                    (`KismetSystemLibrary.PrintString` "Object Delete failed")))
                (else
                  (`KismetSystemLibrary.PrintString` (`KismetStringLibrary.Concat_StrStr` (`|GetEnumeratorNameAsString` _type_type) " was unable to be deleted.")))))))))))

(fn `MenuActive`
  (returns (Active :type Boolean))
  (bind _gameinstance (`self.GameInstance`))
  (`/Engine/EditorBlueprintResources/StandardMacros.IsValid` _gameinstance
    (:`Is Valid`
      (return (or (`/Game/Blueprints/GameInstance/BP_GI_Adventure.IsPauseMenuActive` _gameinstance) (`self.bInMenu`))))
    (:`Is Not Valid`
      (return false))))

(fn `SpawnObjectsFromList`
  (params (Objects :type "Array of GAMEBUILDER_OBJECT Structure"))
  (for _array_element Objects
    (switch `GAMEBUILDER_OBJECT_TYPE` (`.Type` (break `GAMEBUILDER_OBJECT` _array_element))
      (:`INTERACTABLE`
        (`self.RequestSpawnInteractible` (break `GAMEBUILDER_OBJECT` _array_element) (`.Location` (break `GAMEBUILDER_OBJECT` _array_element))))
      (:`SPAWN`
        (`self.RequestSetSpawnLocation` (break `GAMEBUILDER_OBJECT` _array_element) (`.Location` (break `GAMEBUILDER_OBJECT` _array_element)))))))

(fn `UserConstructionScript`)