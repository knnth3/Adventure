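; Player controller for multiplayer adventure mode that handles pause input and tracks the selected pawn.
; Selecting a pawn deselects the previous one and passes the new pawn's ID to BP_ConnectedPlayer as its spectating target.
; SetTargetAsPawn and SetTargetAsFloor switch the opacity material parameter collection's use of character location.
; Once pawn targeting is enabled, Tick keeps writing the selected pawn's location into that collection.
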(event `self.ReceiveBeginPlay`
  (bind _asbp_gi_adventure (cast `/Game/Blueprints/GameInstance/BP_GI_Adventure` (`GameplayStatics.GetGameInstance`)))
  (set `self.GameInstance` _asbp_gi_adventure))

(event `InputAction|Pause`
  (params (Key :type "Key Structure"))
  (bind _gameinstance (`self.GameInstance`))
  (:`Pressed`
    (`/Engine/EditorBlueprintResources/StandardMacros.IsValid` _gameinstance
      (:`Is Valid`
        (`/Game/Blueprints/GameInstance/BP_GI_Adventure.TogglePauseMenu` _gameinstance)))))

(event `/Game/Blueprints/Interfaces/BP_SelectorInterface.OnPawnSelected`
  (params (Pawn :type "/Game/Blueprints/Characters/BP_MapPawn Object Reference"))
  (bind _selectedpawn (`self.SelectedPawn`))
  (`/Engine/EditorBlueprintResources/StandardMacros.IsValid` _selectedpawn
    (:`Is Valid`
      (`/Game/Blueprints/Characters/BP_MapPawn.Deselect` _selectedpawn))
    (:`Is Not Valid`
      _))
  (bind _output_get (set `self.SelectedPawn` Pawn))
  (`/Game/Blueprints/Characters/BP_MapPawn.Select` _output_get)
  (bind _asbp_connected_player (cast `/Game/Blueprints/Characters/BP_ConnectedPlayer` (`GameplayStatics.GetPlayerPawn` 0)))
  (`ConnectedPlayer.SetSpectatingPawn` _asbp_connected_player (`MapPawn.GetPawnID` Pawn)))

(event `self.ReceiveTick`
  (params (DeltaSeconds :type "Float (single-precision)"))
  (bind _selectedpawn (`self.SelectedPawn`))
  (if (`self.bUseTargetLocation`)
    (`/Engine/EditorBlueprintResources/StandardMacros.IsValid` _selectedpawn
      (:`Is Valid`
        (`KismetMaterialLibrary.SetVectorParameterValue` "/Game/Materials/OpacityParameterCollection.OpacityParameterCollection" "CharacterLocation" (`KismetMathLibrary.Conv_VectorToLinearColor` (`self.K2_GetActorLocation` _selectedpawn)))))))

(fn `GetSelectedPawn`
  (returns (Value :type "/Game/Blueprints/Characters/BP_MapPawn Object Reference"))
  (return (`self.SelectedPawn`)))

(fn `OnRep_PlayerName`
  (set `self.bUpdateName` true))

(fn `SetTargetAsFloor`
  (`KismetMaterialLibrary.SetScalarParameterValue` "/Game/Materials/OpacityParameterCollection.OpacityParameterCollection" "bUseCharacterLocation"))

(fn `SetTargetAsPawn`
  (`KismetMaterialLibrary.SetScalarParameterValue` "/Game/Materials/OpacityParameterCollection.OpacityParameterCollection" "bUseCharacterLocation" 1.0)
  (set `self.bUseTargetLocation` true))

(fn `UserConstructionScript`)