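; BP_PC_Adventure_Lobby is the lobby player controller, handling pause input and the player's overhead name.
; It caches BP_GI_Adventure on BeginPlay and toggles that game instance's pause menu when Pause is pressed.
; The PlayerName RepNotify only raises an UpdateName flag.
; Tick then writes the name to the controlled BP_LobbyPawn's overhead text, retrying until that pawn cast succeeds before clearing the flag.
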(event `self.ReceiveBeginPlay`
  (bind _asbp_gi_adventure (cast `/Game/Blueprints/GameInstance/BP_GI_Adventure` (`GameplayStatics.GetGameInstance`)))
  (set `self.GameInstance` _asbp_gi_adventure))

(event `InputAction|Pause`
  (params (Key :type "Key Structure"))
  (bind _gameinstance (`self.GameInstance`))
  (:`Pressed`
    (`/Engine/EditorBlueprintResources/StandardMacros.IsValid` _gameinstance
      (:`Is Valid`
        (`/Game/Blueprints/GameInstance/BP_GI_Adventure.TogglePauseMenu` _gameinstance)))))

(event `self.ReceiveTick`
  (params (DeltaSeconds :type "Float (single-precision)"))
  (if (`self.bUpdateName`)
    (bind _asbp_lobby_pawn (cast `/Game/Blueprints/Characters/BP_LobbyPawn` (`self.K2_GetPawn`)))
    (`/Game/Blueprints/Characters/BP_LobbyPawn.SetOverheadText` _asbp_lobby_pawn (`self.PlayerName`))
    (set `self.bUpdateName` false)))

(fn `OnRep_PlayerName`
  (set `self.bUpdateName` true))

(fn `UserConstructionScript`)