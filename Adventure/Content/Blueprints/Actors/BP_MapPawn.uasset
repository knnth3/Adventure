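; Selectable map pawn that highlights on hover, reports clicks to the player controller and starts with a Basic Sword.
; Statistics events feed health and AC to a world-space health bar, which hides at zero health, scales logarithmically with camera distance and faces the camera in character view.
; A scene capture renders only body, head and equipped weapons.
; Tick rotates TurnVector and keeps the actor on its root bone during physics simulation.
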(event `self.ReceiveBeginPlay`
  (bind _statistics (`self.Statistics`))
  (bind _inventory (`self.Inventory`))
  (`|ExecutionSequence`
    (:`then_0`
      (`SceneComponent.SetAbsolute` (`self.HealthBar`) false true false)
      (bind _ashealth_bar (`self.GetHealthBar`)
        (:`then`
          (`/Game/Blueprints/UI/Common/HealthBar/HealthBar.SetMaxHealth` _ashealth_bar (`StatisticsComponent.GetMaxHealth` _statistics))
          (`/Game/Blueprints/UI/Common/HealthBar/HealthBar.OnHealthChanged` _ashealth_bar (`StatisticsComponent.GetCurrentHealth` _statistics))
          (`/Game/Blueprints/UI/Common/HealthBar/HealthBar.OnACChanged` _ashealth_bar (`StatisticsComponent.GetCurrentAC` _statistics))
          (`InventoryComponent.GiveWeapon` _inventory "Basic Sword" 1)
          (`InventoryComponent.EquipWeapon` _inventory "Basic Sword" true))))
    (:`then_1`
      ;[1 1 1] Add components that can be highlighted when mouse over event or selection
      (`HighlightComponent.AddHighlightableComponents` (`self.Highlight`) (`|MakeArray` (`self.Mesh`) (`self.PawnHeadComponent`) :!type "PrimitiveComponent Object Reference")))))

(event `self.ReceiveActorBeginCursorOver`
  ;[1 1 1] Add components that can be highlighted when mouse over event or selection
  (`HighlightComponent.HighlightObjects` (`self.Highlight`)))

(event `self.ReceiveActorEndCursorOver`
  ;[1 1 1] Add components that can be highlighted when mouse over event or selection
  (`HighlightComponent.DimObjects` (`self.Highlight`)))

(event `self.ReceiveTick`
  (params (DeltaSeconds :type "Float (single-precision)"))
  (bind (_returnvalue_x _returnvalue_y) (`KismetMathLibrary.BreakVector` (`self.ServerOnly_GetDesiredForwardVector`)))
  (bind _mesh (`self.Mesh`))
  (`SceneComponent.K2_SetWorldRotation` (`self.TurnVector`) (`KismetMathLibrary.MakeRotator` 0.0 0.0 (`KismetMathLibrary.DegAtan2` _returnvalue_y _returnvalue_x)) false false)
  (`self.AdjustHealthBarView`)
  (if (`SceneComponent.IsSimulatingPhysics` _mesh "root_jnt")
    (`self.K2_SetActorLocation` (`SceneComponent.GetSocketLocation` _mesh "root_jnt"))))

(event `self.ReceiveActorOnClicked`
  (params (ButtonPressed :type "Key Structure"))
  (message `/Game/Blueprints/Interfaces/BP_SelectorInterface.OnPawnSelected` (`GameplayStatics.GetPlayerController` 0) self))

(event `self.BP_AttackComponent.Event OnAttackEnd`
  (set `self.bIsAttacking` false))

(event `self.Statistics.OnHealthChanged`
  (params (Value :type Integer))
  (bind _ashealth_bar (`self.GetHealthBar`)
    (:`then`
      (`/Game/Blueprints/UI/Common/HealthBar/HealthBar.OnHealthChanged` _ashealth_bar Value)
      (if (<= Value 0)
        (`SceneComponent.SetVisibility` (`self.HealthBar`) false false)))))

(event `self.Statistics.OnACChanged`
  (params (Value :type Integer))
  (bind _ashealth_bar (`self.GetHealthBar`)
    (:`then`
      (`/Game/Blueprints/UI/Common/HealthBar/HealthBar.OnACChanged` _ashealth_bar Value))))

(event `self.Inventory.OnWeaponEquiped`
  (params (RightHand :type Boolean))
  (`SceneCaptureComponent.ShowOnlyActorComponents` (`self.SceneCaptureComponent2D`) (`InventoryComponent.GetWeapon` (`self.Inventory`) RightHand)))

(event `self.Inventory.OnWeaponUnequiped`
  (params (RightHand :type Boolean))
  (`SceneCaptureComponent.RemoveShowOnlyActorComponents` (`self.SceneCaptureComponent2D`) (`InventoryComponent.GetWeapon` (`self.Inventory`) RightHand)))

(fn `AdjustHealthBarView`
  (bind _healthbar (`self.HealthBar`))
  (bind _returnvalue (- (`PlayerCameraManager.GetCameraLocation` (`PlayerController.PlayerCameraManager` (`GameplayStatics.GetPlayerController` 0))) (`SceneComponent.K2_GetComponentLocation` _healthbar)))
  (bind _returnvalue_2 (* (`KismetMathLibrary.Loge` (`KismetMathLibrary.FClamp` (* (/ (`KismetMathLibrary.VSize` _returnvalue) 225.0) 2.718282) 1.0 15.0)) 0.0025))
  (bind _asbp_connected_player (cast `/Game/Blueprints/Actors/BP_ConnectedPlayer` (`GameplayStatics.GetPlayerPawn` 0)))
  (if (`|EnumEquality` (`ConnectedPlayer.GetCameraType` _asbp_connected_player) "CHARACTER")
    (`SceneComponent.K2_SetWorldRotation` _healthbar (`KismetMathLibrary.FindLookAtRotation` (`KismetMathLibrary.MakeVector` 0.0) (`KismetMathLibrary.Normal` _returnvalue)) false false)
    (`SceneComponent.SetRelativeScale3D` _healthbar (`KismetMathLibrary.MakeVector` _returnvalue_2 _returnvalue_2 _returnvalue_2))
    (else
      (`|ExecutionSequence`
        (:`then_0`
          (`/Engine/EditorBlueprintResources/StandardMacros.DoOnce` false
            (:`Completed`
              (set `self.bViewSwitched` true))))
        (:`then_1`
          (if (`self.bViewSwitched`)
            (set `self.bViewSwitched` false)
            (`SceneComponent.K2_SetWorldRotation` _healthbar (struct :`Pitch` 90.0 :`Yaw` 180.0) false false))
          (`SceneComponent.SetRelativeScale3D` _healthbar (`KismetMathLibrary.MakeVector` _returnvalue_2 _returnvalue_2 _returnvalue_2)))))))

(fn `CapturePawn`
  (params (Value :type Boolean))
  (set `SceneCaptureComponent.bCaptureEveryFrame` Value (`self.SceneCaptureComponent2D`)))

(fn `Deselect`
  (`HighlightComponent.DimObjects` (`self.Highlight`)))

(fn `Select`)

(fn `UserConstructionScript`
  (bind _scenecapturecomponent2d (`self.SceneCaptureComponent2D`))
  (`SceneCaptureComponent.ClearShowOnlyComponents` _scenecapturecomponent2d null)
  (`SceneCaptureComponent.ShowOnlyComponent` _scenecapturecomponent2d (`self.Mesh`))
  (`SceneCaptureComponent.ShowOnlyComponent` _scenecapturecomponent2d (`self.PawnHeadComponent`)))