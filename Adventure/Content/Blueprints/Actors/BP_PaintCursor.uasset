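; BP_PaintCursor is a preview cursor actor that shows a mesh and stamps copies of it into the world grid.
; Exposed functions set its mesh and index, visibility, location and rotation, and it caches the first BP_WorldGrid found at BeginPlay.
; AddCopyToWorldGrid passes the mesh index and transform to the grid's ServerOnlyAddBlockingObject, optionally randomizing scale and yaw for each copy.
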(event `self.ReceiveBeginPlay`
  (bind _outactors (`GameplayStatics.GetAllActorsOfClass` "/Game/Blueprints/Grid/BP_WorldGrid.BP_WorldGrid_C"))
  (set `self.WorldGrid` (`|GetArrayItem` _outactors)))

(fn `AddCopyToWorldGrid`
  (locals (FinalScale :type "Vector Structure") (FinalRotation :type "Rotator Structure"))
  (bind _worldgrid (`self.WorldGrid`))
  (`/Engine/EditorBlueprintResources/StandardMacros.IsValid` _worldgrid
    (:`Is Valid`
      (if (`self.bRandomScale`)
        (set `local.FinalScale` (+ (`KismetMathLibrary.MakeVector` 0.8 0.8 0.8) (* (`KismetMathLibrary.RandomFloat`) 0.4)))
        (else
          (bind _output_get (set `local.FinalScale` (.scale (`self.GetTransform`))))))
      (if (`self.bRandomRotation`)
        (set `local.FinalRotation` (`KismetMathLibrary.MakeRotator` 0.0 0.0 (`KismetMathLibrary.RandomFloatInRange` 0.0 359.0)))
        (else
          (bind _output_get_2 (set `local.FinalRotation` (.rotation (`self.GetTransform`))))))
      (`WorldGrid.ServerOnly_AddBlockingObject` _worldgrid (`self.MeshIndex`) (`KismetMathLibrary.MakeTransform` (.location (`self.GetTransform`)) _output_get_2 _output_get)))))

(fn `DisplayCursor`
  (params (Visibility :type Boolean))
  (`SceneComponent.SetVisibility` (`self.StaticMesh`) Visibility false))

(fn `IsVisible`
  (returns (Value :type Boolean))
  (return (`SceneComponent.IsVisible` (`self.StaticMesh`))))

(fn `SetCursorLocation`
  (params (Location :type "Vector Structure"))
  (`self.K2_SetActorLocation` Location))

(fn `SetObjectRotation`
  (params (Rotation :type "Rotator Structure"))
  (`self.K2_SetActorRotation` Rotation true))

(fn `SetStaticMesh`
  (params (MeshIndex :type Byte) (Mesh :type "StaticMesh Object Reference"))
  (set `self.MeshIndex` MeshIndex)
  (`StaticMeshComponent.SetStaticMesh` (`self.StaticMesh`) Mesh))

(fn `UserConstructionScript`)