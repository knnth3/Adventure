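; BP_ConnectedPlayer is the multiplayer player actor that handles camera control, cursor-driven character movement and a grid-snapped movement arrow.
; Input either drives the selected pawn's camera or pans and zooms a spring-arm overview camera, with a material parameter collection tracking the pawn for opacity effects.
; CursorMove moves the character on release, while middle mouse multicasts a free-placed arrow through the server.
; Authority-only keys switch between free-roam and turn-based play.
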(event `self.ReceiveBeginPlay`)

(event `InputAxis|LookUp-Down`
  (params (AxisValue :type "Float (single-precision)"))
  ;[1 1 1] Camera Functions
  (if (`|EnumEquality` (`self.GetCameraType`) "CHARACTER")
    (`self.RotatePawnCameraUpDown` AxisValue (`GameplayStatics.GetWorldDeltaSeconds`))
    (else
      (`self.UpdateOverviewCamera` AxisValue (stale `InputAxis|LookLeft-Right` AxisValue) (stale `InputAxis|Zoom` AxisValue) :!label _label))))

(event `InputAxis|LookLeft-Right`
  (params (AxisValue :type "Float (single-precision)"))
  ;[1 1 1] Camera Functions
  (if (`|EnumEquality` (`self.GetCameraType`) "CHARACTER")
    (`self.RotatePawnCameraLeftRight` AxisValue (`GameplayStatics.GetWorldDeltaSeconds`))
    (else
      (goto _label :!via `LeftRight`))))

(event `InputAxis|Zoom`
  (params (AxisValue :type "Float (single-precision)"))
  ;[1 1 1] Camera Functions
  (if (`|EnumEquality` (`self.GetCameraType`) "CHARACTER")
    (`self.ZoomPawnCameraInOut` AxisValue (`GameplayStatics.GetWorldDeltaSeconds`))
    (else
      (goto _label :!via `Zoom`))))

(event `Key|MiddleMouseButton`
  (params (Key :type "Key Structure"))
  (bind (_world_location _success) (`/Game/Blueprints/Public/PublicFunctions.GetMouseCoordinates3D`))
  ;[1 1 1] Move Controlls
  (:`Pressed`
    (if _success
      (`self.Server_DisplayMovementArrow` true true _world_location)))
  (:`Released`
    (`self.Server_DisplayMovementArrow` false true)))

(event `Key|C`
  (params (Key :type "Key Structure"))
  ;[1 1 1] Camera Functions
  (:`Pressed`
    (`self.SwapCameraView`)))

(event `InputAction|CursorMove`
  (params (Key :type "Key Structure"))
  (bind (_worldlocation _success) (`/Game/Blueprints/Public/PublicFunctions.GetMouseCoordinates3DTrace` false))
  (bind _returnvalue (`GameplayStatics.GetPlayerController` 0))
  ;[1 1 1] Move Controlls
  (:`Pressed`
    (bind _result (message `/Game/Blueprints/Interfaces/BP_SelectorInterface.IsAttacking` _returnvalue))
    (if _result
      (message `/Game/Blueprints/Interfaces/BP_SelectorInterface.SetAttacking` _returnvalue false)
      (else
        (`self.Server_DisplayMovementArrow` true)
        (set `self.bMoveCharacter` true))))
  (:`Released`
    (if (`self.bMoveCharacter`)
      (if _success
        (`self.MovePlayer` _worldlocation)))
    (`self.Server_DisplayMovementArrow` false)
    (set `self.bMoveCharacter` false)))

(event `self.ReceiveTick`
  (params (DeltaSeconds :type "Float (single-precision)"))
  ;[1 1 1] Camera Functions
  (`self.MoveCameraOverview` DeltaSeconds)
  (`self.Event UpdateMovementArrow`)
  (if (`|EnumEquality` (`self.GetCameraType`) "CHARACTER")
    (`self.UpdateOpacityTargetLocation`)
    (else
      (`self.LerpOverviewCamera`))))

(event `self.OnCameraTypeChanged`
  (params (Type :type "CONNECTED_PLAYER_CAMERA Enum" :default "NONE"))
  ;[1 1 1] Camera Functions
  (switch `CONNECTED_PLAYER_CAMERA` Type
    (:`CHARACTER`
      (`self.SetCameraTargetAsPawn`))
    (:`OVERVIEW`
      (`self.SetCameraTargetAsFloor`))))

(event `Key|PageUp`
  (params (Key :type "Key Structure"))
  ;[1 1 1] Change state from free-roam to turn based (Server only)
  (:`Pressed`
    (`/Engine/EditorBlueprintResources/ActorMacros.Switch Has Authority`
      (:`Authority`
        (bind _asbp_gs_multiplayer (cast `/Game/Blueprints/GameStates/BP_GS_Multiplayer` (`GameplayStatics.GetGameState`)))
        (`GS_Multiplayer.SetActivePlayer` _asbp_gs_multiplayer 0)))))

(event `Key|PageDown`
  (params (Key :type "Key Structure"))
  ;[1 1 1] Change state from free-roam to turn based (Server only)
  (:`Pressed`
    (`/Engine/EditorBlueprintResources/ActorMacros.Switch Has Authority`
      (:`Authority`
        (bind _asbp_gs_multiplayer (cast `/Game/Blueprints/GameStates/BP_GS_Multiplayer` (`GameplayStatics.GetGameState`)))
        (`GS_Multiplayer.SetActivePlayer` _asbp_gs_multiplayer -1)))))

(event `Server_DisplayMovementArrow`
  (params (bIsVisible :type Boolean) (bOverrideStart :type Boolean) (StartLocation :type "Vector Structure"))
  (if bOverrideStart
    (`self.Multicast_DisplayMovmentArrow` bIsVisible StartLocation)
    (set `self.bArrowRotatesPawn` false)
    (else
      (`self.DisplayMovementArrow` bIsVisible)
      (set `self.bArrowRotatesPawn` true))))

(event `Multicast_DisplayMovmentArrow`
  (params (bIsVisible :type Boolean) (StartLocation :type "Vector Structure"))
  (`self.DisplayMovementArrow` bIsVisible true StartLocation))

(event `Event UpdateMovementArrow`
  (bind (_world_location _success) (`/Game/Blueprints/Public/PublicFunctions.GetMouseCoordinates3D`))
  (bind _movementarrow (`self.MovementArrow`))
  (bind _movementarrow_2 (`self.MovementArrow`))
  (bind _returnvalue (`GridFunctions.WorldToGridLocation` _world_location))
  (`/Engine/EditorBlueprintResources/StandardMacros.IsValid` _movementarrow
    (:`Is Valid`
      (if (`/Game/Blueprints/Actors/BP_MovementArrow.IsVisible` _movementarrow)
        (if (not (`self.bArrowRotatesPawn`))
          (if _success
            (if (not (`/Game/Blueprints/Public/PublicMacros.isEqual` (`/Game/Blueprints/Actors/BP_MovementArrow.GetEndLocation` _movementarrow_2) _returnvalue))
              (`self.Server_UpdateMovementArrow` _returnvalue)))
          (else
            (`/Game/Blueprints/Actors/BP_MovementArrow.Event UpdateLocation` _movementarrow_2 _returnvalue)))))))

(event `Server_UpdateMovementArrow`
  (params (EndLocation :type "GridCoordinate Structure"))
  (`self.Multicast_UpdateMovementArrow` EndLocation))

(event `Multicast_UpdateMovementArrow`
  (params (EndLocation :type "GridCoordinate Structure"))
  (`/Game/Blueprints/Actors/BP_MovementArrow.Event UpdateLocation` (`self.MovementArrow`) EndLocation))

(fn `DisplayMovementArrow`
  (params (value :type Boolean) (bOverrideCharacterPosition :type Boolean) (Position :type "Vector Structure"))
  (bind _returnvalue (`self.GetSelectedPawn`))
  (bind _movementarrow (`self.MovementArrow`))
  (bind _returnvalue_2 (`|EnumEquality` (`self.GetCameraType`) "OVERVIEW"))
  (`/Engine/EditorBlueprintResources/StandardMacros.IsValid` _movementarrow
    (:`Is Valid`
      (if value
        (if bOverrideCharacterPosition
          (`/Game/Blueprints/Actors/BP_MovementArrow.Event DisplayArrow` _movementarrow true null true (`GridFunctions.WorldToGridLocation` Position) _returnvalue_2)
          (else
            (`/Engine/EditorBlueprintResources/StandardMacros.IsValid` _returnvalue
              (:`Is Valid`
                (`/Game/Blueprints/Actors/BP_MovementArrow.Event DisplayArrow` :`self` _movementarrow :`Display` true :`Pawn` _returnvalue :`bInOverview` _returnvalue_2)))))
        (else
          (`/Game/Blueprints/Actors/BP_MovementArrow.Event DisplayArrow` :`self` _movementarrow :`bInOverview` _returnvalue_2))))))

(fn `LerpOverviewCamera`
  (bind _cameraboom (`self.CameraBoom`))
  (set `SpringArmComponent.TargetArmLength` (`KismetMathLibrary.Lerp` (`SpringArmComponent.TargetArmLength` _cameraboom) (`self.OverviewCameraDistance`) 0.1) _cameraboom))

(fn `MoveCameraOverview`
  (params (deltaTime :type "Float (double-precision)"))
  (`self.K2_AddActorWorldOffset` (* (* (* (`KismetMathLibrary.Normal` (`KismetMathLibrary.MakeVector` (`self.CamYDir`) (`self.CamXDir`))) deltaTime) (`self.OverviewCameraSpeed`)) 100.0)))

(fn `SetCameraTargetAsFloor`
  (`KismetMaterialLibrary.SetScalarParameterValue` "/Game/Materials/MPC/OpacityParameterCollection.OpacityParameterCollection" "bUseCharacterLocation"))

(fn `SetCameraTargetAsPawn`
  (`KismetMaterialLibrary.SetScalarParameterValue` "/Game/Materials/MPC/OpacityParameterCollection.OpacityParameterCollection" "bUseCharacterLocation" 1.0))

(fn `SetMaxZoomDistance`
  (params (Value :type "Float (double-precision)"))
  (set `self.MaxCameraDistance` Value))

(fn `UpdateOpacityTargetLocation`
  (bind _returnvalue (`self.GetSelectedPawn`))
  (`/Engine/EditorBlueprintResources/StandardMacros.IsValid` _returnvalue
    (:`Is Valid`
      (`KismetMaterialLibrary.SetVectorParameterValue` "/Game/Materials/MPC/OpacityParameterCollection.OpacityParameterCollection" "CharacterLocation" (`KismetMathLibrary.Conv_VectorToLinearColor` (`self.K2_GetActorLocation` _returnvalue))))))

(fn `UserConstructionScript`)