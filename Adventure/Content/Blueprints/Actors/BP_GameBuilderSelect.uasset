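; Rectangular area-selection actor for the game builder, stretched from a start corner to a mouse location.
; SetStartLocation places it just above the given point; SetSize scales pivot scenes and moves edge planes, using axis sign to handle negative drags and ignoring near-zero sizes.
; MakeVisible swaps between the mesh and four highlight planes, which ClearHighlight hides.
; Getters report the selection's world-space corners and area in scale units.
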(fn `ClearHighlight`
  (`SceneComponent.SetVisibility` (`self.Plane`) false false)
  (`SceneComponent.SetVisibility` (`self.Plane1`) false false)
  (`SceneComponent.SetVisibility` (`self.Plane3`) false false)
  (`SceneComponent.SetVisibility` (`self.Plane2`) false false))

(fn `GetAreaOfSelected`
  (returns (Area :type "Float (double-precision)"))
  (bind (_relativescale3d_x _relativescale3d_y) (`KismetMathLibrary.BreakVector` (`SceneComponent.RelativeScale3D` (`self.Scene`))))
  (return (`KismetMathLibrary.Abs` (* _relativescale3d_x _relativescale3d_y))))

(fn `GetDimensionsWorldSpace`
  (returns (StartCorner :type "Vector Structure") (EndCorner :type "Vector Structure"))
  (bind _returnvalue (`self.K2_GetActorLocation`))
  (return _returnvalue (+ _returnvalue (* (`SceneComponent.RelativeScale3D` (`self.Scene`)) 100.0))))

(fn `GetDirection`
  (params (Value :type "Float (double-precision)"))
  (returns (Direction :type "Float (double-precision)"))
  (if (== Value 0.0)
    (return 0.0)
    (else
      (return (/ Value (`KismetMathLibrary.Abs` Value))))))

(fn `IsVisible`
  (returns (Visibility :type Boolean))
  (return (`self.bIsVisible`)))

(fn `MakeVisible`
  (params (Value :type Boolean))
  (if (!= Value (`self.bIsVisible`))
    (`SceneComponent.SetVisibility` (`self.StaticMesh`) Value Value)
    (bind _output_get (set `self.bIsVisible` Value))
    (`|ExecutionSequence`
      (:`then_0`
        (bind _returnvalue (not _output_get))
        (`SceneComponent.SetVisibility` (`self.Plane`) _returnvalue false))
      (:`then_1`
        (`SceneComponent.SetVisibility` (`self.Plane1`) _returnvalue false))
      (:`then_2`
        (`SceneComponent.SetVisibility` (`self.Plane2`) _returnvalue false))
      (:`then_3`
        (`SceneComponent.SetVisibility` (`self.Plane3`) _returnvalue false)))))

(fn `SetSize`
  (params (MouseLocation :type "Vector Structure"))
  (locals (NewObjectScale :type "Vector Structure"))
  (bind (_returnvalue_x _returnvalue_y) (`KismetMathLibrary.BreakVector` (`self.K2_GetActorLocation`)))
  (bind _xscene (`self.XScene`))
  (bind (_newobjectscale_x _newobjectscale_y) (`KismetMathLibrary.BreakVector` (`local.NewObjectScale`)))
  (bind (_newobjectscale_x_2 _newobjectscale_y_2) (`KismetMathLibrary.BreakVector` (`local.NewObjectScale`)))
  (bind _direction (`self.GetDirection` _newobjectscale_x_2))
  (if (`self.IsVisible`)
    (bind _output_get (set `local.NewObjectScale` (`KismetMathLibrary.MakeVector` (/ (- MouseLocation_X _returnvalue_x) 100.0) (/ (- MouseLocation_Y _returnvalue_y) 100.0))))
    (`|ExecutionSequence`
      (:`then_0`
        (if (< (`KismetMathLibrary.Abs` (.x _output_get)) 0.01)
          (return)))
      (:`then_1`
        (if (< (`KismetMathLibrary.Abs` (.y _output_get)) 0.01)
          (return)))
      (:`then_2`
        (`SceneComponent.SetRelativeScale3D` (`self.Scene`) (`KismetMathLibrary.MakeVector` _newobjectscale_x_2 _newobjectscale_y_2 1.0))
        (`SceneComponent.SetRelativeScale3D` (`self.YScene`) (`KismetMathLibrary.MakeVector` 1.0 _newobjectscale_y_2 1.0))
        (`SceneComponent.SetRelativeScale3D` _xscene (`KismetMathLibrary.MakeVector` (+ _newobjectscale_x_2 (* 0.1 _direction)) 1.0 1.0))
        (`SceneComponent.K2_SetRelativeLocation` _xscene (`KismetMathLibrary.MakeVector` (* -5.0 _direction)) false false)
        (`SceneComponent.K2_SetRelativeLocation` (`self.Plane1`) (`KismetMathLibrary.MakeVector` (* _newobjectscale_x 100.0) 50.0) false false)
        (`SceneComponent.K2_SetRelativeLocation` (`self.Plane3`) (`KismetMathLibrary.MakeVector` 50.0 (* _newobjectscale_y 100.0)) false false)))))

(fn `SetStartLocation`
  (params (Location :type "Vector Structure"))
  (`self.K2_SetActorLocation` (`KismetMathLibrary.MakeVector` Location_X Location_Y (+ Location_Z 1.0)))
  (`self.SetSize` (`KismetMathLibrary.MakeVector` (+ Location_X 10.0) (+ Location_Y 10.0) Location_Z)))

(fn `UserConstructionScript`)