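; BP_MovementArrow is a grid movement indicator that draws an arrow from a pawn or fixed start cell to a target cell, labeled in feet.
; DisplayArrow sets visibility, start and view mode, while UpdateLocation moves the end.
; While visible, Tick places the actor at the end, yaws it along the path, stretches the base and shrinks the head when short.
; The label counts Manhattan squares at 5ft each, facing the camera outside overview.
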(event `self.ReceiveTick`
  (params (DeltaSeconds :type "Float (single-precision)"))
  (bind _pawn (`self.Pawn`))
  (bind _arrow (`self.Arrow`))
  (bind _distancetextrenderer (`self.DistanceTextRenderer`))
  (bind (_returnvalue_x _returnvalue_y) (`KismetMathLibrary.BreakVector` (`GridFunctions.GridToWorldLocation` (`self.EndLocation`))))
  (bind (_returnvalue_x_2 _returnvalue_y_2) (`KismetMathLibrary.BreakVector` (`GridFunctions.GridToWorldLocation` (`self.StartLocation`))))
  (bind (_returnvalue_x_3 _returnvalue_y_3) (`KismetMathLibrary.BreakVector2D` (- (`KismetMathLibrary.MakeVector2D` _returnvalue_x _returnvalue_y) (`KismetMathLibrary.MakeVector2D` _returnvalue_x_2 _returnvalue_y_2))))
  (bind (_x _y) (`KismetMathLibrary.BreakVector2D` (/ (`self.Distance`) 152.399002)))
  (bind _returnvalue (`KismetMathLibrary.VSize2D` (`KismetMathLibrary.MakeVector2D` _returnvalue_x_3 _returnvalue_y_3)))
  (bind _returnvalue_2 (/ _returnvalue 146.0))
  (if (`self.bArrowVisible`)
    (`|ExecutionSequence`
      (:`then_0`
        (if (and (not (`self.bUseLocation`)) (`KismetSystemLibrary.IsValid` _pawn))
          (set `self.StartLocation` (`GridFunctions.WorldToGridLocation` (`self.K2_GetActorLocation` _pawn))))
        (`self.K2_SetActorLocation` (`KismetMathLibrary.MakeVector` _returnvalue_x _returnvalue_y 20.0))
        (set `self.Distance` (`KismetMathLibrary.MakeVector2D` _returnvalue_x_3 _returnvalue_y_3))
        (`self.K2_SetActorRotation` (`KismetMathLibrary.MakeRotator` 0.0 0.0 (`KismetMathLibrary.DegAtan2` _returnvalue_y_3 _returnvalue_x_3)))
        (`SceneComponent.SetRelativeScale3D` (`self.Base`) (`KismetMathLibrary.MakeVector` (- (/ _returnvalue 100.0) 0.5) 1.0 1.0))
        (if (< _returnvalue_2 1.0)
          (`SceneComponent.SetWorldScale3D` _arrow (`KismetMathLibrary.MakeVector` _returnvalue_2 _returnvalue_2 1.0))
          (else
            (`SceneComponent.SetWorldScale3D` _arrow (1.0 1.0 1.0)))))
      (:`then_1`
        (if (`self.bInOverview`)
          (`SceneComponent.K2_SetWorldRotation` _distancetextrenderer (struct :`Pitch` 90.0 :`Yaw` 180.0) false false)
          (else
            (`SceneComponent.K2_SetWorldRotation` _distancetextrenderer (`KismetMathLibrary.MakeRotFromX` (- (`self.K2_GetActorLocation` (`GameplayStatics.GetPlayerCameraManager` 0)) (`SceneComponent.K2_GetComponentLocation` _distancetextrenderer))) false false)))
        (`TextRenderComponent.K2_SetText` _distancetextrenderer (`KismetTextLibrary.Conv_StringToText` (`KismetStringLibrary.Concat_StrStr` (`KismetStringLibrary.Conv_IntToString` (* (+ (`KismetMathLibrary.Abs_Int` (`KismetMathLibrary.FTrunc` _x)) (`KismetMathLibrary.Abs_Int` (`KismetMathLibrary.FTrunc` _y))) 5)) " ft")))))))

(event `Event DisplayArrow`
  (params (Display :type Boolean) (Pawn :type "Actor Object Reference") (bUseLocationOverride :type Boolean) (Location :type "GridCoordinate Structure") (bInOverview :type Boolean))
  (`self.DisplayArrow` Display Pawn bUseLocationOverride Location bInOverview))

(event `Event UpdateLocation`
  (params (EndLocation :type "GridCoordinate Structure"))
  (set `self.EndLocation` EndLocation))

(fn `DisplayArrow`
  (params (Display :type Boolean) (Pawn :type "Actor Object Reference") (bUseLocationInstead :type Boolean) (Location :type "GridCoordinate Structure") (bInOverview :type Boolean))
  (`SceneComponent.SetVisibility` (`self.Arrow`) Display true)
  (set `self.bArrowVisible` Display)
  (set `self.Pawn` Pawn)
  (set `self.bUseLocation` bUseLocationInstead)
  (bind _output_get (set `self.StartLocation` Location))
  (set `self.bInOverview` bInOverview)
  (set `self.EndLocation` _output_get))

(fn `GetEndLocation`
  (returns (EndLocation :type "GridCoordinate Structure"))
  (return (`self.EndLocation`)))

(fn `IsVisible`
  (returns (bArrowVisible :type Boolean))
  (return (`self.bArrowVisible`)))

(fn `UserConstructionScript`)