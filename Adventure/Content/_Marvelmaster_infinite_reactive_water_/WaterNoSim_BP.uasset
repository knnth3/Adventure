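; WaterNoSim_BP is a non-simulated water tile that shows a simplified water material on its static mesh.
; Its construction script disables actor and component ticking and applies that material.
; An unconnected timeline graph holds logic to swap it for a WaterSim_BP when the selected pawn comes within SpawnSimTileDist, passing on MasterIndex and that distance.
; As wired, that swap never runs.
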(fn `UserConstructionScript`
  (`ActorComponent.SetComponentTickEnabled` (`self.meshcenter`) false)
  (`ActorComponent.SetComponentTickEnabled` (`self.StaticMesh`) false)
  ;[1 1 1] Get Water Material simple version from master
  (`self.SetActorTickEnabled` false)
  (`PrimitiveComponent.SetMaterial` (`self.StaticMesh`) 0 (`self.WaterMaterialSimplyfied`)))