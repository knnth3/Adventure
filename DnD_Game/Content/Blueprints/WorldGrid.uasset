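; WorldGrid is an actor that defines the map's grid dimensions and shares them with materials through the MapSettingsPC parameter collection.
; On BeginPlay, SetGridDivisons stores the dimensions and writes them to the collection's grid vector parameter.
; It also returns a cell size from actor scale over divisions, multiplied by CellDivisionToPercentage, whose math is unconnected.
; BeginPlay passes zero cell divisions and ignores that result.
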(event `self.ReceiveBeginPlay`
  (`self.SetGridDivisons` (`self.Grid Dimensions`) (0.0 0.0)))

(fn `SetGridDivisons`
  (params (`Grid Divisions` :type "Vector2D Structure") (`Cell Divisions` :type "Vector2D Structure"))
  (returns (`Cell Dimensions` :type "Vector2D Structure"))
  (bind (_returnvalue_x _returnvalue_y) (`KismetMathLibrary.BreakVector` (`self.GetActorScale3D`)))
  (set `self.Grid Dimensions` (`KismetMathLibrary.MakeVector2D` `Grid Divisions_X` `Grid Divisions_Y`))
  (`KismetMaterialLibrary.SetVectorParameterValue` "/Game/Blueprints/Materials/MapSettingsPC.MapSettingsPC" "Grid Dimensions (x,y)" (make `LinearColor` `Grid Divisions_X` `Grid Divisions_Y`))
  (return (* (`KismetMathLibrary.MakeVector2D` (/ _returnvalue_x `Grid Divisions_X`) (/ _returnvalue_y `Grid Divisions_Y`)) (`self.CellDivisionToPercentage` `Cell Divisions`))))

(fn `UserConstructionScript`)