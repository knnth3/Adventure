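; Editor camera that either glides freely on Up/Down and Left/Right input or snaps to a target's location each tick.
; SetTarget switches it to following; the file shows no detach.
; Free movement integrates velocity per axis from input acceleration, adding friction when input stops or reverses, with a stopping dead zone and optional terminal-speed clamp.
; BeginPlay derives friction as twice the X acceleration, and Tick applies the resulting position without sweeping.
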(event `self.ReceiveBeginPlay`
  (bind _acceleration_x (`KismetMathLibrary.BreakVector` (`self.Acceleration`)))
  (set `self.FrictionDeceleration` (* _acceleration_x 2.0)))

(event `self.ReceiveTick`
  (params (DeltaSeconds :type "Float (single-precision)"))
  (if (`self.isAttatched`)
    (`self.MoveWithTarget`)
    (else
      (bind _new_position (`self.GetNextPosition` (`self.Direction`) DeltaSeconds))
      (`self.K2_SetActorLocation` _new_position false true))))

(event `InputAxis|Up/Down`
  (params (AxisValue :type "Float (single-precision)"))
  (bind (_direction_x _direction_y _direction_z) (`KismetMathLibrary.BreakVector` (`self.Direction`)))
  (set `self.Direction` (`KismetMathLibrary.MakeVector` AxisValue _direction_y _direction_z)))

(event `InputAxis|Left/Right`
  (params (AxisValue :type "Float (single-precision)"))
  (bind (_direction_x _direction_y _direction_z) (`KismetMathLibrary.BreakVector` (`self.Direction`)))
  (set `self.Direction` (`KismetMathLibrary.MakeVector` _direction_x AxisValue _direction_z)))

(fn `CalculateVelocity`
  (params (Direction :type "Vector Structure") (`Initial Velocity` :type "Vector Structure") (`Acceleration Constant` :type "Vector Structure") (`Delta Seconds` :type "Float (double-precision)") (`Friction Coeficient` :type "Float (double-precision)") (`Terminal Velocity` :type "Float (double-precision)") (`Stopping Dead Zone` :type "Float (double-precision)"))
  (returns (`Final Velocity` :type "Vector Structure"))
  ;[1 1 1] Calculate new velocty based off given parameters
  (bind _final_velocity (`self.GetVelocityComponent` Direction_X `Initial Velocity_X` `Acceleration Constant_X` `Delta Seconds` `Friction Coeficient` `Stopping Dead Zone` `Terminal Velocity`))
  (bind _final_velocity_2 (`self.GetVelocityComponent` Direction_Y `Initial Velocity_Y` `Acceleration Constant_Y` `Delta Seconds` `Friction Coeficient` `Stopping Dead Zone` `Terminal Velocity`))
  (bind _final_velocity_3 (`self.GetVelocityComponent` Direction_Z `Initial Velocity_Z` `Acceleration Constant_Z` `Delta Seconds` `Friction Coeficient` `Stopping Dead Zone` `Terminal Velocity`))
  (return (`KismetMathLibrary.MakeVector` _final_velocity _final_velocity_2 _final_velocity_3)))

(fn `GetAccelerationComponent`
  (params (Direction :type "Float (double-precision)") (Speed :type "Float (double-precision)") (acceleration :type "Float (double-precision)") (`Friction Coeficient` :type "Float (double-precision)"))
  (returns (`New Acceleration` :type "Float (double-precision)") (Decelerating :type Boolean))
  (bind _returnvalue (* Direction acceleration))
  ;[1 1 1] Switches between friction acc and user controlled acc
  (if (== Direction 0.0)
    (bind _friction (`self.GetFriction` Speed `Friction Coeficient`))
    (return _friction true)
    (else
      (bind _same (`self.InSameDirection` Speed _returnvalue))
      (if _same
        (return _returnvalue false)
        (else
          (bind _friction_2 (`self.GetFriction` Speed `Friction Coeficient`))
          (return (+ _friction_2 _returnvalue) true))))))

(fn `GetFriction`
  (params (speed :type "Float (double-precision)") (`Friction Coeficient` :type "Float (double-precision)"))
  (returns (Friction :type "Float (double-precision)"))
  (`/Engine/EditorBlueprintResources/StandardMacros.CompareFloat` speed
    (:`>`
      (return (* -1.0 `Friction Coeficient`)))
    (:`==`
      (return (* 0 `Friction Coeficient`)))
    (:`<`
      (return `Friction Coeficient`))))

(fn `GetVelocityComponent`
  (params (Direction :type "Float (double-precision)") (`Initial Velocity` :type "Float (double-precision)") (Acceleration :type "Float (double-precision)") (Time :type "Float (double-precision)") (`Friction Coeficient` :type "Float (double-precision)") (DeadZone :type "Float (double-precision)") (`Terminal Velocity` :type "Float (double-precision)"))
  (returns (`Final Velocity` :type "Float (double-precision)"))
  ;[1 1 1] Calculates Velocity component (x,y,or z) using v = v + at
  (bind (_new_acceleration _decelerating) (`self.GetAccelerationComponent` Direction `Initial Velocity` Acceleration `Friction Coeficient`))
  (bind _returnvalue (+ `Initial Velocity` (* _new_acceleration Time)))
  (bind _returnvalue_2 (`KismetMathLibrary.Abs` _returnvalue))
  (if (and _decelerating (< _returnvalue_2 DeadZone))
    (return 0.0)
    (elif (<= `Terminal Velocity` 0.0)
      (return _returnvalue)
      (elif (< _returnvalue_2 `Terminal Velocity`)
        (return _returnvalue)
        (else
          (return (* (`KismetMathLibrary.FMin` _returnvalue_2 `Terminal Velocity`) (/ _returnvalue _returnvalue_2))))))))

(fn `InSameDirection`
  (params (`Value 1` :type "Float (double-precision)") (`Value 2` :type "Float (double-precision)"))
  (returns (same :type Boolean))
  (`/Engine/EditorBlueprintResources/StandardMacros.CompareFloat` `Value 1`
    (:`>`
      (`/Engine/EditorBlueprintResources/StandardMacros.CompareFloat` `Value 2`
        (:`>`
          _)
        (:`==`
          _)
        (:`<`
          (return false)))
      (return true))
    (:`==`
      (`/Engine/EditorBlueprintResources/StandardMacros.CompareFloat` `Value 2`
        (:`>`
          _)
        (:`==`
          _)
        (:`<`
          _))
      (return true))
    (:`<`
      (`/Engine/EditorBlueprintResources/StandardMacros.CompareFloat` `Value 2`
        (:`>`
          (return false))
        (:`==`
          _)
        (:`<`
          _))
      (return true))))

(fn `MoveWithTarget`
  (`self.K2_SetActorLocation` (`self.K2_GetActorLocation` (`self.Target`))))

(fn `SetTarget`
  (params (Target :type "Actor Object Reference"))
  (returns (Success :type Boolean))
  (set `self.Target` Target)
  (bind _output_get (set `self.isAttatched` true))
  (return _output_get))

(fn `UserConstructionScript`)