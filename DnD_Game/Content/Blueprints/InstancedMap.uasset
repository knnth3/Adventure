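; InstancedMap is a Blueprint that builds a grid-based level from a saved level design file at BeginPlay.
; It spawns a LevelDesignLog, loads the named file through it, stores map name and grid dimensions, then spawns each logged mesh at its grid location.
; SpawnObject batches meshes into one Instanced Static Mesh component per mesh type, created on first use and cached in a map.
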(event `self.ReceiveBeginPlay`
  (bind _returnvalue (`|SpawnActorFromClass` "/Script/DnD_Game.LevelDesignLog" (`KismetMathLibrary.MakeTransform` (0.0 0.0 0.0)) "AlwaysSpawn" "OverrideRootScale" null null))
  (set `self.Log` _returnvalue)
  (bind _success (`self.LoadMap`))
  (if _success
    (`KismetSystemLibrary.PrintString` "Map Load Success")
    (else
      (`KismetSystemLibrary.PrintString` "Map Load Failed"))))

(fn `CreateNewMeshInstance`
  (params (`Static Mesh` :type "StaticMesh Object Reference"))
  (returns (Instance :type "InstancedStaticMeshComponent Object Reference"))
  (bind _returnvalue (`AddComponent|NODE_AddInstancedStaticMeshComponent-2`))
  (`BlueprintMapLibrary.Map_Add` (`self.InstancedMeshTypes`) `Static Mesh` _returnvalue)
  (`StaticMeshComponent.SetStaticMesh` _returnvalue `Static Mesh`)
  (return _returnvalue))

(fn `LoadMap`
  (returns (Success :type Boolean))
  (bind _log (`self.Log`))
  (bind (_name _rows _columns) (`LevelDesignLog.GetLevelInfo` _log))
  (bind _returnvalue (`LevelDesignLog.LoadLogFrom` _log (`self.FileName`)))
  (if _returnvalue
    (set `self.MapName` _name)
    (set `self.Grid Dimensions` (`KismetMathLibrary.MakeVector2D` (`KismetMathLibrary.Conv_IntToDouble` _rows) (`KismetMathLibrary.Conv_IntToDouble` _columns)))
    (for _index (range (`LevelDesignLog.GetActorCount` _log))
      (bind _returnvalue_2 (`LevelDesignLog.GetMeshOf` _log _index))
      (if (!= _returnvalue_2 null)
        (`self.SpawnObject` _returnvalue_2 (`.position` (break `Decorative` (`LevelDesignLog.GetInfoOf` _log _index))))))
    (return true)
    (else
      (return false))))

(fn `SpawnObject`
  (params (`Static Mesh` :type "StaticMesh Object Reference") (`Grid Location` :type "Vector2D Structure"))
  (bind (_value _returnvalue) (`BlueprintMapLibrary.Map_Find` (`self.InstancedMeshTypes`) `Static Mesh`))
  (bind _world_location (`/Game/Blueprints/WorldGridConversionFunctions.GridLocationToWorld` (`self.CellDimensions`) `Grid Location`))
  (if _returnvalue
    (`InstancedStaticMeshComponent.AddInstanceWorldSpace` _value (`KismetMathLibrary.MakeTransform` _world_location))
    (else
      (bind _instance (`self.CreateNewMeshInstance` `Static Mesh`))
      (`InstancedStaticMeshComponent.AddInstance` _instance (`KismetMathLibrary.MakeTransform` _world_location)))))

(fn `UserConstructionScript`)