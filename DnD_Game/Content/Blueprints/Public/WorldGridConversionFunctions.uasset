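; Blueprint function library that converts between world locations and 2D grid cells, with cursor-trace and centimeter/meter helpers.
; World-to-grid rounds X and Y away from zero to cell multiples, then divides by cell dimensions.
; Grid-to-world returns cell centers at Z zero, using each coordinate's sign for the half-cell offset, which assumes nonzero indices.
; The cursor helper traces a given channel and returns the hit flattened to Z zero with a success flag.
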(fn `CentimetersToMeters`
  (params (Centimeters :type "Float (double-precision)"))
  (returns (Meters :type "Float (double-precision)"))
  (return (/ Centimeters 100.0)))

(fn `GetMouseCoordinates3D`
  (params (`Trace Channel` :type "ETraceTypeQuery Enum" :default "TraceTypeQuery1"))
  (returns (`World Location` :type "Vector Structure") (Success :type Boolean))
  (bind (_hitresult _returnvalue) (`PlayerController.GetHitResultUnderCursorByChannel` (`GameplayStatics.GetPlayerController` null) `Trace Channel` false))
  (if _returnvalue
    (return (`KismetMathLibrary.MakeVector` (.x (`.Location` (`GameplayStatics.BreakHitResult` _hitresult))) (.y (`.Location` (`GameplayStatics.BreakHitResult` _hitresult)))) true)
    (else
      (return (0.0 0.0 0.0) false))))

(fn `GridLocationToWorld`
  (params (`Cell Dimensions` :type "Vector2D Structure") (`Grid Location` :type "Vector2D Structure"))
  (returns (`World Location` :type "Vector Structure"))
  (return (`KismetMathLibrary.Conv_Vector2DToVector` (- (* (`KismetMathLibrary.MakeVector2D` `Cell Dimensions_X` `Cell Dimensions_Y`) (`KismetMathLibrary.MakeVector2D` `Grid Location_X` `Grid Location_Y`)) (`KismetMathLibrary.MakeVector2D` (* (/ `Grid Location_X` (`KismetMathLibrary.Abs` `Grid Location_X`)) (/ `Cell Dimensions_X` 2.0)) (* (/ `Grid Location_Y` (`KismetMathLibrary.Abs` `Grid Location_Y`)) (/ `Cell Dimensions_Y` 2.0)))))))

(fn `MetersToCentimeters`
  (params (Meters :type "Float (double-precision)"))
  (returns (Centimeters :type "Float (double-precision)"))
  (return (* Meters 100.0)))

(fn `RoundToNearest`
  (params (Value :type "Float (double-precision)") (Divisor :type "Float (double-precision)"))
  (returns (`New Position` :type "Float (double-precision)"))
  (bind _returnvalue (mod Value Divisor))
  (bind _returnvalue_2 (- Value _returnvalue))
  ;[1 1 1] Rounds a number to the biggest value divisible by Divisor with zero remainder  EX: 4.7->5.0 if divisor = 1
  (`/Engine/EditorBlueprintResources/StandardMacros.CompareFloat` _returnvalue
    (:`>`
      (return (+ _returnvalue_2 Divisor)))
    (:`==`
      (return Value))
    (:`<`
      (return (- _returnvalue_2 Divisor)))))

(fn `WorldLocationToGrid`
  (params (`Cell Dimensions` :type "Vector2D Structure") (`World Location` :type "Vector Structure"))
  (returns (`Grid Location` :type "Vector2D Structure"))
  (return (`KismetMathLibrary.MakeVector2D` (/ (`self.RoundToNearest` `World Location_X` `Cell Dimensions_X`) `Cell Dimensions_X`) (/ (`self.RoundToNearest` `World Location_Y` `Cell Dimensions_Y`) `Cell Dimensions_Y`))))