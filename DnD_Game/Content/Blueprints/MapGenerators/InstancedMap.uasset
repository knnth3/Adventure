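; Grid-based map actor that builds a level from a saved LevelDesignLog file and moves player pawns across it.
; On BeginPlay it spawns a scaled floor plane, groups decorations into one instanced mesh component per mesh type, then creates a Grid2D and the player pawns.
; Unoccupied cells near a player display as instanced move markers.
; Destinations go through Grid2D pathfinding into a step queue that Tick feeds to the idle selected pawn.
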(event EventBeginPlay
  (bind _returnvalue (Game|SpawnActorfromClass "/Script/DnD_Game.LevelDesignLog" (Math|Transform|MakeTransform "0, 0, 0" "0, 0, 0" "1,1,1") "AlwaysSpawn" 0 0))
  (Variables|MapInfo|SetLog _returnvalue)
  (bind _success (Construction|LoadMap))
  (if _success
    (Construction|CreateGrid)
    (Construction|SpawnActors)))

(event EventTick
  (params (DeltaSeconds :type Float%20%28single-precision%29))
  (PlayerInfo|SetPlayerMoveInstruction (Variables|Players|GetSelectedPlayerIndex)))

(fn ConstructionScript)

(fn CreateNewMeshInstance
  (params (Static%20Mesh :type Static%20Mesh%20Object%20Reference))
  (bind _returnvalue (AddComponent|AddInstancedStaticMeshComponent false))
  (Collision|SetCollisionResponsetoChannel _returnvalue "ECC_GameTraceChannel1" "ECR_Ignore")
  (Utilities|Map|Add (Variables|MapInfo|GetInstancedMeshTypes) Static%20Mesh _returnvalue)
  (Components|StaticMesh|SetStaticMesh _returnvalue Static%20Mesh)
  (return _returnvalue))

(fn LoadMap
  (bind _log (Variables|MapInfo|GetLog))
  (bind (_name _rows _columns) (Class|LevelDesignLog|GetLevelInfo _log))
  (bind _returnvalue (Class|LevelDesignLog|LoadLogfrom _log (Variables|MapInfo|GetFileName)))
  (if _returnvalue
    (Variables|MapInfo|SetMapName _name)
    (Variables|MapInfo|SetGrid%20Dimensions (Math|Vector2D|MakeVector2D (Math|Conversions|ToFloat(Integer) _rows) (Math|Conversions|ToFloat(Integer) _columns)))
    (Construction|SpawnFloor (Variables|MapInfo|GetGrid%20Dimensions) (Variables|MapInfo|GetCellDimensions))
    (for _index (range 0 (- (Class|LevelDesignLog|GetActorCount _log) 1))
      (if (!= (Class|LevelDesignLog|GetMeshOf _log _index) 0)
        (Construction|SpawnDecorations (Class|LevelDesignLog|GetMeshOf _log _index) (.position (.obj (Class|LevelDesignLog|GetInfoOf _log _index))))))
    (return true)
    (else
      (return false))))

(fn SpawnDecorations
  (params (Static%20Mesh :type Static%20Mesh%20Object%20Reference) (Grid%20Location :type Vector%202D%20Structure))
  (bind _instancedmeshtypes (Variables|MapInfo|GetInstancedMeshTypes))
  (bind _celldimensions (Variables|MapInfo|GetCellDimensions))
  (bind _centimeters (CallFunction|MeterstoCentimeters (.y _celldimensions)))
  (bind _centimeters_2 (CallFunction|MeterstoCentimeters (.x _celldimensions)))
  (bind (_value _returnvalue) (Utilities|Map|Find _instancedmeshtypes Static%20Mesh))
  (bind _world_location (CallFunction|GridLocationtoWorld (Math|Vector2D|MakeVector2D _centimeters_2 _centimeters) Grid%20Location))
  (if _returnvalue
    (Class|InstancedStaticMeshComponent|AddInstanceWorldSpace _value (Math|Transform|MakeTransform _world_location "0, 0, 0" "1,1,1"))
    (else
      (bind _instance (Construction|CreateNewMeshInstance Static%20Mesh))
      (Collision|SetCollisionResponsetoAllChannels _instance "ECR_Ignore")
      (Class|InstancedStaticMeshComponent|AddInstanceWorldSpace _instance (Math|Transform|MakeTransform _world_location "0, 0, 0" "1,1,1")))))

(fn SpawnFloor
  (params (GridDimensions :type Vector%202D%20Structure) (CellDimensions :type Vector%202D%20Structure))
  (bind _returnvalue (* GridDimensions CellDimensions))
  (bind _returnvalue_2 (AddComponent|AddStaticMeshComponent false (Math|Transform|MakeTransform (Math|Vector|MakeVector (CallFunction|MeterstoCentimeters (/ (.x _returnvalue) -2.0)) (CallFunction|MeterstoCentimeters (/ (.y _returnvalue) 2.0)) 0.0) "0, 0, 0" (Math|Vector|MakeVector (.x _returnvalue) (.y _returnvalue) 1.0))))
  (Components|StaticMesh|SetStaticMesh _returnvalue_2 "/Engine/BasicShapes/Plane.Plane")
  (Collision|SetCollisionResponsetoChannel _returnvalue_2 "ECC_GameTraceChannel3" "ECR_Ignore"))

(fn SpawnActors
  (for _index (range 1 (Variables|Players|GetNumberOfPlayers))
    (bind _returnvalue (Game|SpawnActorfromClass "/Game/Blueprints/Actors/ControllableMapPawn.ControllableMapPawn_C" (Math|Transform|MakeTransform "-600.000000,300.000000, 0" "0, 0, 0" "1,1,1") "AdjustIfPossibleButAlwaysSpawn" 0 0))
    (|Ingnorealltracechannels _returnvalue)
    (Utilities|Array|Insert (Variables|Players|GetLoadedPlayers) _returnvalue (- _index 1))))

(fn GetPlayer
  (params (Index :type Integer))
  (bind _loadedplayers (Variables|Players|GetLoadedPlayers))
  (bind _returnvalue (Utilities|Array|Length _loadedplayers))
  (if (and (Math|Integer|InRange(Integer) Index 0 _returnvalue true false) (!= _returnvalue 0))
    (return (Utilities|Array|Get(acopy) _loadedplayers Index) true)
    (else
      (return 0 false))))

(fn GetPlayerLocation
  (params (index :type Integer))
  (bind (_character _success) (PlayerInfo|GetPlayer index))
  (if _success
    (return (Transformation|GetActorLocation _character) true)
    (else
      (return "0, 0, 0" false))))

(fn SetPlayerDestination
  (params (Index :type Integer) (Location :type Vector))
  (bind (_character _success) (PlayerInfo|GetPlayer Index))
  (bind _grid (Utilities|CMWorldtoGrid Location))
  (bind _returnvalue (Transformation|GetActorLocation _character))
  (bind _grid_2 (Utilities|CMWorldtoGrid _returnvalue))
  (if _success
    (Utilities|Array|Clear (Variables|Players|GetCurrentMoveInstructions))
    (if (Math|Vector|Equal(Vector) _grid_2 _grid 0.0001)
      (Default|SetDestination _character Location false)
      (elif (Variables|Players|GetbShowingMoveOptions)
        (|PathFind _character _grid_2 _grid)
        (Variables|Players|SetSelectedPlayerIndex Index)))))

(fn ShowPlayerMoveLocations
  (params (Index :type Integer))
  (bind (_position _success) (PlayerInfo|GetPlayerLocation2D Index))
  (bind _grid_dimensions (Variables|MapInfo|GetGrid%20Dimensions))
  (if (not (Variables|Players|GetbShowingMoveOptions))
    (Variables|Players|SetbShowingMoveOptions true)
    (if (and _success (.Success (PlayerInfo|GetPlayer Index)))
      (Rendering|Material|SetVectorParameterValue "/Game/Blueprints/Materials/MovementPanelColorParams.MovementPanelColorParams" "Center" (Math|Conversions|ToLinearColor(Vector) (Utilities|GridtoWorld (Math|Vector2D|MakeVector2D (.x _position) (.y _position)))) :!class /Script/Engine.KismetMaterialLibrary)
      (for _index (range -3 3)
        (if (Math|Integer|InRange(Integer) (+ _index (Math|Float|Truncate (.x _position))) (Math|Float|Truncate (* (.x _grid_dimensions) -1.0)) 0 true false)
          (for _index_2 (range -3 3)
            (if (Math|Integer|InRange(Integer) (+ _index_2 (Math|Float|Truncate (.y _position))) 0 (Math|Float|Truncate (.y _grid_dimensions)) false)
              (if (not (Class|LevelDesignLog|IsGridSpaceOccupied (Variables|MapInfo|GetLog) (Math|Vector2D|MakeVector2D (Math|Conversions|ToFloat(Integer) (+ _index (Math|Float|Truncate (.x _position)))) (Math|Conversions|ToFloat(Integer) (+ _index_2 (Math|Float|Truncate (.y _position)))))))
                (Components|InstancedStaticMesh|AddInstance (Variables|Default|GetPlayerMovePositions) (Math|Transform|MakeTransform (Math|Vector|MakeVector (CallFunction|MeterstoCentimeters (.x (CallFunction|GridLocationtoWorld (Variables|MapInfo|GetCellDimensions) (Math|Vector2D|MakeVector2D (Math|Conversions|ToFloat(Integer) (+ _index (Math|Float|Truncate (.x _position)))) (Math|Conversions|ToFloat(Integer) (+ _index_2 (Math|Float|Truncate (.y _position)))))))) (CallFunction|MeterstoCentimeters (.y (CallFunction|GridLocationtoWorld (Variables|MapInfo|GetCellDimensions) (Math|Vector2D|MakeVector2D (Math|Conversions|ToFloat(Integer) (+ _index (Math|Float|Truncate (.x _position)))) (Math|Conversions|ToFloat(Integer) (+ _index_2 (Math|Float|Truncate (.y _position)))))))) 0.0) "0, 0, 0" "1.500000,1.500000,1"))))))))))

(fn GetPlayerLocation2D
  (params (Index :type Integer))
  (bind (_newparam _success) (PlayerInfo|GetPlayerLocation Index))
  (bind _celldimensions (Variables|MapInfo|GetCellDimensions))
  (if _success
    (return (CallFunction|WorldLocationtoGrid (Math|Vector2D|MakeVector2D (CallFunction|MeterstoCentimeters (.x _celldimensions)) (CallFunction|MeterstoCentimeters (.y _celldimensions))) _newparam) true)
    (else
      (return "" false))))

(fn HidePlayerMoveLocations
  (if (Variables|Players|GetbShowingMoveOptions)
    (Variables|Players|SetbShowingMoveOptions false)
    (Components|InstancedStaticMesh|ClearInstances (Variables|Default|GetPlayerMovePositions))))

(fn MoveOptionsDisplayed
  (return (Variables|Players|GetbShowingMoveOptions)))

(fn CreateGrid
  (bind _grid_dimensions (Variables|MapInfo|GetGrid%20Dimensions))
  (bind _returnvalue (Game|SpawnActorfromClass "/Script/DnD_Game.Grid2D" (Math|Transform|MakeTransform "0, 0, 0" "0, 0, 0" "1,1,1") "AlwaysSpawn" 0 0))
  (bind _output_get (Variables|MapInfo|SetGrid _returnvalue))
  (Class|Grid2D|MakeGrid _output_get (Math|Float|Truncate (.x _grid_dimensions)) (Math|Float|Truncate (.y _grid_dimensions))))

(fn SetPlayerMoveInstruction
  (params (Index :type Integer))
  (bind (_character _success) (PlayerInfo|GetPlayer Index))
  (bind _currentmoveinstructions (Variables|Players|GetCurrentMoveInstructions))
  (if (!= (Utilities|Array|Length _currentmoveinstructions) 0)
    (if _success
      (if (not (Default|IsMoving _character))
        (Default|SetDestination _character (Utilities|GridtoWorld (Utilities|Array|Get(acopy) _currentmoveinstructions)) false)
        (Utilities|Array|RemoveIndex _currentmoveinstructions)))))