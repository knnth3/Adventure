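; Decoration actor that shows an assignable mesh, snaps to grid cells and reports its name and position.
; Selection toggles a highlight plane and custom depth, while Tick pulses the outline glow through the PostProcessOutline parameter collection, which also receives the color.
; MakeTranslucent hides the model outright on camera overlap, and a Tick-driven countdown restores its visibility.
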(event `self.ReceiveBeginPlay`
  ;[1 1 1] Set up defaults
  (bind _returnvalue (`PrimitiveComponent.CreateDynamicMaterialInstance` (`self.HighlightPlane`) 0 "/Game/Blueprints/Materials/FloorSelect.FloorSelect"))
  (set `self.HilightMaterial` _returnvalue)
  (`self.RemoveAsActive`))

(event `self.ReceiveTick`
  (params (DeltaSeconds :type "Float (single-precision)"))
  (bind _elapsedtime (`self.ElapsedTime`))
  (`self.MakeOpaque` DeltaSeconds)
  ;[1 1 1] Pulse if Selected
  (if (`self.Selected`)
    (`KismetMaterialLibrary.SetScalarParameterValue` "/Game/Blueprints/Materials/PostProcessOutline.PostProcessOutline" "Glow" (`KismetMathLibrary.Lerp` (`self.MinGlow`) (`self.Max Glow`) (`self.GetPeriod`)))
    (if (>= _elapsedtime (`KismetMathLibrary.MultiplyByPi` 2.0))
      (set `self.ElapsedTime` 0.0))
    (set `self.ElapsedTime` (+ _elapsedtime (* DeltaSeconds (`self.PulseSpeedScalar`))))))

(fn `GetInfo`
  (returns (Info :type "Decorative Structure"))
  (return (`self.ObjectInfo`)))

(fn `MakeOpaque`
  (params (`Elapsed Time` :type "Float (double-precision)"))
  (if (`self.bCameraOverlap`)
    (`/Engine/EditorBlueprintResources/StandardMacros.CompareFloat` (`self.InvisibleTimer`)
      (:`>`
        (set `self.InvisibleTimer` (- (`self.InvisibleTimer`) `Elapsed Time`)))
      (:`==`
        (`SceneComponent.SetVisibility` (`self.Model`) true false :!label _label)
        (set `self.bCameraOverlap` false)
        (set `self.InvisibleTimer` 0.0))
      (:`<`
        (goto _label)))))

(fn `MakeTranslucent`
  (`/Engine/EditorBlueprintResources/StandardMacros.CompareFloat` (`self.InvisibleTimer`)
    (:`>`
      _)
    (:`==`
      (`SceneComponent.SetVisibility` (`self.Model`) false false))
    (:`<`
      _))
  (set `self.bCameraOverlap` true)
  (set `self.InvisibleTimer` (`self.TimeHidden`)))

(fn `Move`
  (params (`Cell Dimensions` :type "Vector2D Structure") (`Grid Position` :type "Vector2D Structure"))
  (bind _objectinfo_name (break `Decorative` (`self.ObjectInfo`)))
  (set `self.ObjectInfo` (make `Decorative` _objectinfo_name `Grid Position`))
  (`self.K2_SetActorLocation` (`/Game/Blueprints/WorldGridConversionFunctions.GridLocationToWorld` `Cell Dimensions` `Grid Position`) false true))

(fn `RemoveAsActive`
  (bind _output_get (set `self.Selected` false))
  (`SceneComponent.SetVisibility` (`self.HighlightPlane`) _output_get false)
  (`PrimitiveComponent.SetRenderCustomDepth` (`self.HighlightPlane`) false)
  (if (`self.bHasModel`)
    (`PrimitiveComponent.SetRenderCustomDepth` (`self.Model`) false)))

(fn `SetAsActive`
  (bind _output_get (set `self.Selected` true))
  (`SceneComponent.SetVisibility` (`self.HighlightPlane`) _output_get false)
  (`KismetSystemLibrary.PrintString` "Activated")
  (`PrimitiveComponent.SetRenderCustomDepth` (`self.HighlightPlane`) true)
  (if (`self.bHasModel`)
    (`PrimitiveComponent.SetRenderCustomDepth` (`self.Model`) true)))

(fn `SetColor`
  (params (Color :type "Vector Structure"))
  (if (== Color (`self.GlowColor`))
    _
    (else
      _))
  (bind _output_get (set `self.GlowColor` Color))
  (`KismetMaterialLibrary.SetVectorParameterValue` "/Game/Blueprints/Materials/PostProcessOutline.PostProcessOutline" "Color" (`KismetMathLibrary.Conv_VectorToLinearColor` _output_get)))

(fn `SetMesh`
  (params (Mesh :type "StaticMesh Object Reference"))
  (returns (`Return Value` :type Boolean))
  (bind (_objectinfo_name _objectinfo_position) (break `Decorative` (`self.ObjectInfo`)))
  (bind _model (`self.Model`))
  (bind _returnvalue (`StaticMeshComponent.SetStaticMesh` _model Mesh))
  (set `self.ObjectInfo` (make `Decorative` (`KismetSystemLibrary.GetDisplayName` Mesh) _objectinfo_position))
  (bind _output_get (set `self.bHasModel` _returnvalue))
  (`SceneComponent.SetVisibility` _model true false)
  (return _output_get))

(fn `UserConstructionScript`)