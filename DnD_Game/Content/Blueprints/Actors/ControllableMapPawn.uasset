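; Map pawn that glides in a straight line to a given destination while turning its skeletal mesh to face it, or only turns on request.
; SetDestination stores the target and calls SetRotation, which derives a yaw from the direction using atan2.
; Tick teleports the root at constant speed without sweeping, snapping to a stop within an approximation radius.
; A timeline, restarted on each new heading, drives a shortest-path rotation lerp.
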(event `self.ReceiveTick`
  (params (DeltaSeconds :type "Float (single-precision)"))
  (`|ExecutionSequence`
    (:`then_0`
      (if (`self.bMoveCharacter`)
        (`self.MoveCharacter` DeltaSeconds)))
    (:`then_1`
      (if (`self.bRotateCharacter`)
        (if (`self.bResetRotation`)
          (set `self.bResetRotation` false)
          (bind (_direction _alpha) (`Timeline|Rotation Timeline` :!via `PlayFromStart` :!label _label)
            (:`Update`
              (`self.RotateCharacter` _alpha)))
          (else
            (goto _label)))))))

(event `SetDestination2`
  (params (Location :type "Vector Structure") (OnlyRotateCharacter :type Boolean))
  (`self.SetDestination` Location OnlyRotateCharacter))

(fn `IsMoving`
  (returns (`Return Value` :type Boolean))
  (return (`self.bMoveCharacter`)))

(fn `MoveCharacter`
  (params (`Delta Seconds` :type "Float (double-precision)"))
  (bind _destination (`self.Destination`))
  (bind _scene (`self.Scene`))
  (bind _returnvalue (`SceneComponent.K2_GetComponentLocation` _scene))
  (if (`self.bMoveCharacter`)
    (if (== _destination _returnvalue :`ErrorTolerance` (`self.MoveAproximationRadius`))
      (bind _output_get (set `self.Destination` _returnvalue))
      (set `self.bMoveCharacter` false)
      (`SceneComponent.K2_SetWorldLocation` _scene _output_get false true)
      (else
        (`SceneComponent.K2_SetWorldLocation` _scene (+ (* (* (`KismetMathLibrary.Normal` (- _destination _returnvalue)) (`/Game/Blueprints/Public/WorldGridConversionFunctions.MetersToCentimeters` (`self.MoveSpeed`))) `Delta Seconds`) _returnvalue) false true)))))

(fn `RotateCharacter`
  (params (Alpha :type "Float (double-precision)"))
  (if (`self.bRotateCharacter`)
    (`SceneComponent.K2_SetRelativeRotation` (`self.SkeletalMesh`) (`KismetMathLibrary.RLerp` (`self.PreviousRotation`) (`self.CurrentRotation`) Alpha true) false false)))

(fn `SetDestination`
  (params (Location :type "Vector Structure") (OnlyRotateCharacter :type Boolean))
  (bind _returnvalue (`SceneComponent.K2_GetComponentLocation` (`self.SkeletalMesh`)))
  (if OnlyRotateCharacter
    (`self.SetRotation` (`KismetMathLibrary.Normal` (- Location _returnvalue)))
    (else
      (bind _output_get (set `self.Destination` Location))
      (set `self.bMoveCharacter` true)
      (`self.SetRotation` (`KismetMathLibrary.Normal` (- _output_get _returnvalue))))))

(fn `SetRotation`
  (params (Direction :type "Vector Structure"))
  (bind _returnvalue (mod (+ (`KismetMathLibrary.DegAtan2` Direction_Y Direction_X) 270.0) 360.0))
  (set `self.bRotateCharacter` true)
  (set `self.bResetRotation` true)
  (`/Engine/EditorBlueprintResources/StandardMacros.CompareFloat` _returnvalue
    (:`>`
      (set `self.CurrentRotation` (`KismetMathLibrary.MakeRotator` 0.0 0.0 _returnvalue) :!label _label)
      (set `self.PreviousRotation` (`SceneComponent.RelativeRotation` (`self.SkeletalMesh`))))
    (:`==`
      (goto _label))
    (:`<`
      (set `self.CurrentRotation` (`KismetMathLibrary.MakeRotator` 0.0 0.0 (+ _returnvalue 360.0))))))

(fn `UserConstructionScript`)