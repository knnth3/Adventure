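; Player character Blueprint with an orbit-and-zoom camera on a spring arm.
; Input axes rotate the arm in yaw and pitch and adjust its length, clamping pitch and zoom.
; Each tick, a trace from camera to skeletal mesh makes a hit Decoration translucent so it stops blocking the view.
; SetDestination stores a target and raises a flag for per-tick movement, but the MoveCharacter function is still empty.
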(event `InputAxis|Left/Right`
  (params (AxisValue :type "Float (single-precision)"))
  (`self.Move Camera Left/Right` AxisValue))

(event `InputAxis|Up/Down`
  (params (AxisValue :type "Float (single-precision)"))
  (`self.Move Camera Up/Down` AxisValue))

(event `InputAxis|In/Out`
  (params (AxisValue :type "Float (single-precision)"))
  (`self.Move Camera In/Out` AxisValue))

(event `self.ReceiveTick`
  (params (DeltaSeconds :type "Float (single-precision)"))
  (`self.RemoveDecorationFromView`)
  (if (`self.bMoveCharacter`)
    (`self.Move Character`)))

(fn `Move Camera In/Out`
  (params (`Axis Value` :type "Float (double-precision)"))
  (bind _springarm (`self.SpringArm`))
  (bind _result (`/Engine/EditorBlueprintResources/StandardMacros.NegateFloat` `Axis Value`)
    (:`  `
      (`/Engine/EditorBlueprintResources/StandardMacros.CompareFloat` _result
        (:`>`
          _)
        (:`<`
          _))
      (set `SpringArmComponent.TargetArmLength` (`KismetMathLibrary.FClamp` (+ (* `Axis Value` (`self.CameraMoveSpeed`)) (`SpringArmComponent.TargetArmLength` _springarm)) (`self.MinCameraZoom`) (`self.MaxCameraZoom`)) _springarm))))

(fn `Move Camera Left/Right`
  (params (`Axis Value` :type "Float (double-precision)"))
  (bind _result (`/Engine/EditorBlueprintResources/StandardMacros.NegateFloat` `Axis Value`)
    (:`  `
      (`/Engine/EditorBlueprintResources/StandardMacros.CompareFloat` _result
        (:`>`
          _)
        (:`<`
          _))
      (`SceneComponent.K2_AddRelativeRotation` (`self.SpringArm`) (`KismetMathLibrary.MakeRotator` 0.0 0.0 (* _result (`self.CameraMoveSpeed`))) false false))))

(fn `Move Camera Up/Down`
  (params (`Axis Value` :type "Float (double-precision)"))
  (bind _springarm (`self.SpringArm`))
  (bind (_relativerotation_roll _relativerotation_pitch _relativerotation_yaw) (`KismetMathLibrary.BreakRotator` (`SceneComponent.RelativeRotation` _springarm)))
  (bind _result (`/Engine/EditorBlueprintResources/StandardMacros.NegateFloat` `Axis Value`)
    (:`  `
      (`/Engine/EditorBlueprintResources/StandardMacros.CompareFloat` _result
        (:`>`
          _)
        (:`<`
          _))
      (`SceneComponent.K2_AddRelativeRotation` _springarm (`KismetMathLibrary.MakeRotator` 0.0 (* _result (`self.CameraMoveSpeed`))) false false)
      (`SceneComponent.K2_SetRelativeRotation` _springarm (`KismetMathLibrary.MakeRotator` _relativerotation_roll (`KismetMathLibrary.FClamp` _relativerotation_pitch -85.0 0.0) _relativerotation_yaw) false false))))

(fn `Move Character`)

(fn `RemoveDecorationFromView`
  (locals (NewLocalVar_0 :type "Array of EObjectTypeQuery Enum"))
  (bind (_outhit _returnvalue) (`KismetSystemLibrary.LineTraceSingleForObjects` :`Start` (`SceneComponent.K2_GetComponentLocation` (`self.Camera`)) :`End` (`SceneComponent.K2_GetComponentLocation` (`self.SkeletalMesh`)) :`ObjectTypes` (`local.NewLocalVar_0`) :`DrawTime` 3.0))
  (if _returnvalue
    (bind _asdecoration (cast `/Game/Blueprints/Decoration` (`.HitActor` (`GameplayStatics.BreakHitResult` _outhit))))
    (`/Game/Blueprints/Decoration.MakeTranslucent` _asdecoration)))

(fn `SetDestination`
  (params (Destination :type "Vector Structure"))
  (set `self.Destination` Destination)
  (set `self.bMoveCharacter` true))

(fn `UserConstructionScript`)