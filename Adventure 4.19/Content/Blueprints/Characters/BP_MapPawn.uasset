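; BP_MapPawn is a map pawn with a separate head actor and an adjustable boom camera.
; On BeginPlay it spawns BP_MapPawn_Head and attaches it to the PawnBody's NA_Head socket, then destroys it on EndPlay.
; Zoom and rotation events scale axis input by delta time and CameraSettings speeds, clamping arm length and pitch while leaving yaw free.
; BeginMove is an empty event, and the construction script does nothing.
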(event `self.BeginMove`)

(event `self.ReceiveBeginPlay`
  (bind _returnvalue (`|SpawnActorFromClass` "/Game/Blueprints/Characters/BP_MapPawn_Head.BP_MapPawn_Head_C" (`KismetMathLibrary.MakeTransform` (0.0 0.0 0.0)) "AlwaysSpawn" "OverrideRootScale" null null))
  (bind _output_get (set `self.HeadActor` _returnvalue))
  (`self.K2_AttachToComponent` _output_get (`self.PawnBody`) "NA_Head" "KeepRelative" "SnapToTarget" "KeepWorld" true))

(event `self.ReceiveEndPlay`
  (params (EndPlayReason :type "EEndPlayReason Enum" :default "Destroyed"))
  (`self.K2_DestroyActor` (`self.HeadActor`)))

(event `self.ZoomInOut`
  (params (AxisValue :type "Float (single-precision) (by ref)") (DeltaTime :type "Float (single-precision) (by ref)"))
  (bind _cameraboom (`self.CameraBoom`))
  (bind (_angularvelocity _zoomspeed _maxuprotation _maxdownrotation _maxinzoom _maxoutzoom) (break `CameraSettings` (`self.CameraSettings`)))
  ;[1 1 1] Camera Controls
  (if (!= AxisValue 0.0)
    (set `SpringArmComponent.TargetArmLength` (`KismetMathLibrary.FClamp` (+ (`SpringArmComponent.TargetArmLength` _cameraboom) (* AxisValue DeltaTime _zoomspeed -1.0)) _maxinzoom _maxoutzoom) _cameraboom)))

(event `self.RotateUpDown`
  (params (AxisValue :type "Float (single-precision) (by ref)") (DeltaTime :type "Float (single-precision) (by ref)"))
  (bind _cameraboom (`self.CameraBoom`))
  (bind (_angularvelocity _zoomspeed _maxuprotation _maxdownrotation) (break `CameraSettings` (`self.CameraSettings`)))
  (bind (_returnvalue_roll _returnvalue_pitch _returnvalue_yaw) (`KismetMathLibrary.BreakRotator` (`SceneComponent.K2_GetComponentRotation` _cameraboom)))
  ;[1 1 1] Camera Controls
  (if (!= AxisValue 0.0)
    (`SceneComponent.K2_SetWorldRotation` _cameraboom (`KismetMathLibrary.MakeRotator` _returnvalue_roll (`KismetMathLibrary.ClampAngle` (- _returnvalue_pitch (* AxisValue DeltaTime _angularvelocity)) _maxuprotation _maxdownrotation) _returnvalue_yaw) false false)))

(event `self.RotateLeftRight`
  (params (AxisValue :type "Float (single-precision) (by ref)") (DeltaTime :type "Float (single-precision) (by ref)"))
  (bind _cameraboom (`self.CameraBoom`))
  (bind (_returnvalue_roll _returnvalue_pitch _returnvalue_yaw) (`KismetMathLibrary.BreakRotator` (`SceneComponent.K2_GetComponentRotation` _cameraboom)))
  ;[1 1 1] Camera Controls
  (if (!= AxisValue 0.0)
    (`SceneComponent.K2_SetWorldRotation` _cameraboom (`KismetMathLibrary.MakeRotator` _returnvalue_roll _returnvalue_pitch (- _returnvalue_yaw (* AxisValue DeltaTime (`.AngularVelocity` (break `CameraSettings` (`self.CameraSettings`)))))) false false)))

(fn `UserConstructionScript`)