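; Player pawn for turn-based play, with character and overview camera modes and click-to-move.
; Look and zoom axes drive either the pawn camera functions or a RotateOverviewCamera macro, depending on camera type.
; Despite its name, that macro pans the actor along world axes and changes boom length, pausing while the controller's menu is active.
; C swaps views with a fade, cursor select traces a destination for pawn 0, and P calls ServerEndTurn.
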(event `self.ReceiveBeginPlay`
  (bind _asbp_pc_adventure_editor (cast `/Game/Blueprints/PlayerControllers/BP_PC_Adventure_Editor` (`GameplayStatics.GetPlayerController` 0)))
  (set `self.MyController` _asbp_pc_adventure_editor))

(event `InputAxis|LookUp-Down`
  (params (AxisValue :type "Float (single-precision)"))
  ;[1 1 1] Camera Switcher Controls
  (if (`|EnumEquality` (`self.GetCameraType`) "CHARACTER")
    (`self.RotatePawnCameraUpDown` AxisValue (`GameplayStatics.GetWorldDeltaSeconds`))
    (else
      (`self.RotateOverviewCamera` AxisValue (stale `InputAxis|LookLeft-Right` AxisValue) (stale `InputAxis|Zoom` AxisValue) :!label _label))))

(event `InputAxis|LookLeft-Right`
  (params (AxisValue :type "Float (single-precision)"))
  ;[1 1 1] Camera Switcher Controls
  (if (`|EnumEquality` (`self.GetCameraType`) "CHARACTER")
    (`self.RotatePawnCameraLeftRight` AxisValue (`GameplayStatics.GetWorldDeltaSeconds`))
    (else
      (goto _label :!via `LeftRight`))))

(event `InputAxis|Zoom`
  (params (AxisValue :type "Float (single-precision)"))
  ;[1 1 1] Camera Switcher Controls
  (if (`|EnumEquality` (`self.GetCameraType`) "CHARACTER")
    (`self.ZoomPawnCameraInOut` AxisValue (`GameplayStatics.GetWorldDeltaSeconds`))
    (else
      (goto _label :!via `Zoom`))))

(event `Key|C`
  (params (Key :type "Key Structure"))
  ;[1 1 1] Camera Switcher Controls
  (:`Pressed`
    (`self.SwapCameraView` (`self.CameraFadeTime`))
    (`KismetSystemLibrary.PrintString` "Switch")))

(event `InputAction|CursorSelect` :paused true
  (params (Key :type "Key Structure"))
  (bind (_world_location _success) (`/Game/Blueprints/Public/PublicFunctions.GetMouseCoordinates3D` "TraceTypeQuery3" true))
  (:`Pressed`
    (if _success
      (`self.MovePlayer` _world_location 0))))

(event `Key|P`
  (params (Key :type "Key Structure"))
  (:`Pressed`
    (`self.Server_EndTurn`)))

(fn `UserConstructionScript`)