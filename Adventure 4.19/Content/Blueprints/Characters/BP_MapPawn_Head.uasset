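; BP_MapPawn_Head is a head piece for a map pawn that swaps its static mesh between boy and girl head variants.
; SetMesh picks the boy or girl mesh list by a flag, applies the indexed mesh to the Head component and stores the index.
; An out-of-range or unchanged index prints an on-screen "Not In bounds" message and returns false.
; The event graph and construction script are empty.
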(event `self.ReceiveBeginPlay`)

(fn `SetMesh`
  (params (MeshIndex :type Integer) (Boy :type Boolean))
  (returns (Success :type Boolean))
  (bind _head (`self.Head`))
  (bind _g_headmeshlist (`self.G_HeadMeshList`))
  (bind _b_headmeshlist (`self.B_HeadMeshList`))
  (bind _returnvalue (`KismetArrayLibrary.Array_Length` _b_headmeshlist))
  (bind _returnvalue_2 (!= MeshIndex (`self.MeshIndex`)))
  (if Boy
    (if (and (> _returnvalue MeshIndex) _returnvalue_2)
      (bind _returnvalue_3 (`StaticMeshComponent.SetStaticMesh` _head (`|GetArrayItem` _b_headmeshlist MeshIndex)))
      (set `self.MeshIndex` MeshIndex)
      (return _returnvalue_3)
      (else
        _))
    (elif (and _returnvalue_2 (> (`KismetArrayLibrary.Array_Length` _g_headmeshlist) MeshIndex))
      (bind _returnvalue_4 (`StaticMeshComponent.SetStaticMesh` _head (`|GetArrayItem` _g_headmeshlist MeshIndex)))
      (set `self.MeshIndex` MeshIndex)
      (return _returnvalue_4)
      (else
        _)))
  (`KismetSystemLibrary.PrintString` (`KismetStringLibrary.Concat_StrStr` "Not In bounds: " (`KismetStringLibrary.Conv_IntToString` MeshIndex) " Current Index = " (`KismetStringLibrary.Conv_IntToString` _returnvalue)) true true (struct :`R` 1.0 :`G` 0.156877 :`A` 1.0) 10.0)
  (return false))

(fn `UserConstructionScript`)