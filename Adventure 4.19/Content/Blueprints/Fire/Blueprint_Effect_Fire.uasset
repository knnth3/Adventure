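; Fire effect Blueprint that flickers a point light by animating its intensity.
; A timeline's FireIntensity track sets the PointLight intensity on each update, with Tick driving it forward or in reverse according to the Reverse flag.
; When the timeline finishes, it waits a random delay, then randomly picks a direction and restarts from that end to vary the flicker.
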(event `self.ReceiveTick`
  (params (DeltaSeconds :type "Float (single-precision)"))
  (if (`self.bReverse`)
    (bind (_direction _fire_intensity) (`Timeline|Timeline_0` :!via `Reverse` :!label _label)
      (:`Update`
        (`LightComponent.SetIntensity` (`self.PointLight`) _fire_intensity))
      (:`Finished`
        (`KismetSystemLibrary.Delay` (* (`KismetMathLibrary.RandomFloat`) 5.0))
        (if (>= (`KismetMathLibrary.RandomFloat`) 0.5)
          (set `self.bReverse` false)
          (goto _label :!via `PlayFromStart`)
          (else
            (set `self.bReverse` true)
            (goto _label :!via `ReverseFromEnd`)))))
    (else
      (goto _label))))

(fn `UserConstructionScript`)