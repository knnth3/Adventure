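; LevelSaveGame is a save object that stores a level's map name, objects and map size.
; Save writes the object itself to a slot named after MapName, so each map name gets its own save.
; Load reads the named slot, copies those three fields into the current instance, and returns false if the slot is missing, invalid or of another class.
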(fn `Load`
  (params (SlotName :type String))
  (returns (success :type Boolean))
  (bind _returnvalue (`GameplayStatics.DoesSaveGameExist` SlotName))
  (if _returnvalue
    (bind _returnvalue_2 (`GameplayStatics.LoadGameFromSlot` SlotName))
    (`/Engine/EditorBlueprintResources/StandardMacros.IsValid` _returnvalue_2
      (:`Is Valid`
        (bind _aslevel_save_game (cast `/Game/Blueprints/SaveGameFiles/LevelSaveGame` _returnvalue_2)
          (:`then`
            (set `self.MapName` (`/Game/Blueprints/SaveGameFiles/LevelSaveGame.MapName` _aslevel_save_game))
            (set `self.Objects` (`/Game/Blueprints/SaveGameFiles/LevelSaveGame.Objects` _aslevel_save_game))
            (set `self.MapSize` (`/Game/Blueprints/SaveGameFiles/LevelSaveGame.MapSize` _aslevel_save_game))
            (return true))
          (:`CastFailed`
            (return false))))
      (:`Is Not Valid`
        (return false)))
    (else
      (return false))))

(fn `Save`
  (returns (success :type Boolean))
  (bind _returnvalue (`GameplayStatics.SaveGameToSlot` self (`self.MapName`)))
  (return _returnvalue))