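; BP_GM_Lobby is the multiplayer lobby game mode, giving the local host a BP_Lobby_Host pawn and other players the default pawn.
; BeginPlay spawns PlayerStarts from StartLocations and moves the first player's pawn to a fixed spot; EndPlay destroys those starts.
; ChoosePlayerStart increments a player counter, then uses it to index the spawned starts.
; PostLogin copies the player's name onto BP_PC_Adventure_Multiplayer and prints it.
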(event `self.ReceiveBeginPlay`
  (for _array_element (`self.StartLocations`)
    (bind _returnvalue (`|SpawnActorFromClass` "/Script/Engine.PlayerStart" (`KismetMathLibrary.MakeTransform` _array_element (struct :`Yaw` 90.0)) "Undefined" "OverrideRootScale" null null))
    (`KismetArrayLibrary.Array_Add` (`self.Spawners`) _returnvalue))
  (`self.K2_SetActorLocation` (`Controller.K2_GetPawn` (`GameplayStatics.GetPlayerController` 0)) (-1000.0 0.0 250.0) false false))

(event `self.ReceiveEndPlay`
  (params (EndPlayReason :type "EEndPlayReason Enum" :default "Destroyed"))
  (for _array_element (`self.Spawners`)
    (`/Engine/EditorBlueprintResources/StandardMacros.IsValid` _array_element
      (:`Is Valid`
        (`self.K2_DestroyActor` _array_element)))))

(event `self.K2_PostLogin`
  (params (NewPlayer :type "PlayerController Object Reference"))
  (bind _returnvalue (`PlayerState.GetPlayerName` (`Controller.PlayerState` NewPlayer)))
  (bind _asbp_pc_adventure_multiplayer (cast `/Game/Blueprints/PlayerControllers/BP_PC_Adventure_Multiplayer` NewPlayer))
  (set `/Game/Blueprints/PlayerControllers/BP_PC_Adventure_Multiplayer.PlayerName` (`KismetTextLibrary.Conv_StringToText` _returnvalue) _asbp_pc_adventure_multiplayer)
  (`KismetSystemLibrary.PrintString` _returnvalue))

(fn `ChoosePlayerStart`
  (params (Player :type "Controller Object Reference"))
  (returns (ReturnValue :type "Actor Object Reference"))
  (bind _numplayers (`self.NumPlayers`))
  (bind _spawners (`self.Spawners`))
  (if (< _numplayers (`KismetArrayLibrary.Array_Length` _spawners))
    (set `self.NumPlayers` (+ _numplayers 1))
    (return (`|GetArrayItem` _spawners _numplayers))))

(fn `GetDefaultPawnClassForController`
  (params (InController :type "Controller Object Reference"))
  (returns (ReturnValue :type "Object Class Reference"))
  (bind _returnvalue (`parent.GetDefaultPawnClassForController` InController))
  (if (`Controller.IsLocalPlayerController` InController)
    (return "/Game/Blueprints/Characters/BP_Lobby_Host.BP_Lobby_Host_C")
    (else
      (return _returnvalue))))

(fn `UserConstructionScript`)