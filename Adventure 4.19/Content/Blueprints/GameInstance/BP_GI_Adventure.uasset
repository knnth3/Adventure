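; Game instance for the adventure game that holds the loaded level save and owns the pause menu.
; Init creates the PauseMenu widget once, and helper functions query its active state or toggle it through Activate and Deactivate.
; LoadSave reads a named slot and caches it as a LevelSaveGame for GetSave, printing a message if the slot is missing, invalid or the wrong type.
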(event `self.ReceiveInit`
  (bind _returnvalue (`|CreateWidget` "/Game/Blueprints/UI/Multiplayer/PauseMenu.PauseMenu_C" (`GameplayStatics.GetPlayerController` 0)))
  (set `self.PauseMenu` _returnvalue))

(fn `GetSave`
  (returns (NewParam :type "/Game/Blueprints/SaveGameFiles/LevelSaveGame Object Reference"))
  (return (`self.CurrenLoadedSave`)))

(fn `IsPauseMenuActive`
  (returns (Value :type Boolean))
  (bind _pausemenu (`self.PauseMenu`))
  (`/Engine/EditorBlueprintResources/StandardMacros.IsValid` _pausemenu
    (:`Is Valid`
      (return (`W_PauseMenu.IsActive` _pausemenu)))
    (:`Is Not Valid`
      (return false))))

(fn `LoadSave`
  (params (SlotName :type String))
  (bind _returnvalue (`GameplayStatics.DoesSaveGameExist` SlotName))
  (if _returnvalue
    (bind _returnvalue_2 (`GameplayStatics.LoadGameFromSlot` SlotName))
    (`/Engine/EditorBlueprintResources/StandardMacros.IsValid` _returnvalue_2
      (:`Is Valid`
        (bind _aslevel_save_game (cast `/Game/Blueprints/SaveGameFiles/LevelSaveGame` _returnvalue_2)
          (:`then`
            (set `self.CurrenLoadedSave` _aslevel_save_game))
          (:`CastFailed`
            (`KismetSystemLibrary.PrintString` "Save game was not a map in GI"))))
      (:`Is Not Valid`
        (`KismetSystemLibrary.PrintString` "Invalid Save loaded in GI")))
    (else
      (`KismetSystemLibrary.PrintString` "Savegame not found while loading in GI"))))

(fn `TogglePauseMenu`
  (bind _pausemenu (`self.PauseMenu`))
  (if (`W_PauseMenu.IsActive` _pausemenu)
    (`W_PauseMenu.Deactivate` _pausemenu)
    (else
      (`W_PauseMenu.Activate` _pausemenu))))